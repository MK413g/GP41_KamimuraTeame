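; BP_MagatamaBit is a magatama actor whose mesh and point light change color with its Move flag.
; Tick picks a random Color data table row when Move turns true, using a DoOnce to hold it until Move turns false.
; While Move is false, it applies the gray row, blacks out the light and resets the DoOnce.
; The construction script creates the dynamic material; the yaw rotation logic is disconnected.
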(event `self.ReceiveBeginPlay`)

(event `self.ReceiveTick`
  (params (DeltaSeconds :type "Float (single-precision)"))
  (if (`self.Move`)
    (`/Engine/EditorBlueprintResources/StandardMacros.DoOnce` false :!label _label
      (:`Completed`
        (bind _returnvalue (`|GetDataTableRow` "/Game/Main/DataTable/Color.Color" (`KismetArrayLibrary.Array_Random` (`self.ColorName`)))
          (:`then`
            (bind (_r _g _b) (break `/Game/Main/DataTable/DataTableStruct/ColorTable` _returnvalue))
            (`MaterialInstanceDynamic.SetVectorParameterValue` (`self.DMI_Random`) "BaseColor" (`KismetMathLibrary.MakeColor` _r _g _b))
            (`LightComponent.SetLightColor` (`self.PointLight`) (make `LinearColor` _r _g _b 1.0) true)))))
    (else
      (bind _returnvalue_2 (`|GetDataTableRow` "/Game/Main/DataTable/Color.Color" "gray")
        (:`then`
          (bind (_r_2 _g_2 _b_2) (break `/Game/Main/DataTable/DataTableStruct/ColorTable` _returnvalue_2))
          (`MaterialInstanceDynamic.SetVectorParameterValue` (`self.DMI_Random`) "BaseColor" (`KismetMathLibrary.MakeColor` _r_2 _g_2 _b_2))
          (`LightComponent.SetLightColor` (`self.PointLight`) (struct :`A` 1.0) true)
          (goto _label :!via `Reset`))))))

(fn `UserConstructionScript`
  (bind _returnvalue (`PrimitiveComponent.CreateDynamicMaterialInstance` (`self.Magatama`) 0 null "BaseColor"))
  (set `self.DMI_Random` _returnvalue))