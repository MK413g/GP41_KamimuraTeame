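; Magatama weapon that the player picks up on overlap, fires with the Shot input, and that damages and knocks back enemies on hit.
; Shots aim through a forward line trace from the player, while Tick updates movement and clears hit flags so damage triggers only on fresh hits.
; Pickup and post-hit reset toggle the minimap marker, MagatamaBit movement and field-specific Niagara or Cascade effect.
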(event `InputAction|Shot` :consume false
  (params (Key :type "Key Structure"))
  (bind _returnvalue (`GameplayStatics.GetPlayerPawn` 0))
  (bind _shot (`self.shot`))
  (bind _returnvalue_2 (`self.K2_GetActorLocation` _returnvalue))
  ;[1 1 1] 弾発射処理
  (:`Pressed`
    (if (`MainGameEndManager.GetGameEnd`)
      _
      (elif (`self.GetShotAngle` _returnvalue)
        (bind _outhit (`KismetSystemLibrary.LineTraceSingleForObjects` _returnvalue_2 (+ _returnvalue_2 (* (`self.GetActorForwardVector` _returnvalue) 2000.0)) (`self.Object Types`)))
        (bind (_bblockinghit _binitialoverlap _time _distance _location) (`GameplayStatics.BreakHitResult` _outhit))
        (if _bblockinghit
          (`self.SetupShot` (* (`KismetMathLibrary.Normal` (- _location (`self.K2_GetActorLocation`))) _shot))
          (else
            (`self.SetupShot` (* (`KismetMathLibrary.Normal` (`self.GetActorForwardVector` (`GameplayStatics.GetPlayerPawn` 0))) _shot))))
        (`SoundManagerBase.PlaySound2D` "/Game/Main/Sound/SE/ShotMagatama/ShotMagatama_Cue.ShotMagatama_Cue" "BGM" 1.0 1.0 0.0 null null)))))

(event `self.Sphere1.OnComponentBeginOverlap`
  (params (OverlappedComponent :type "PrimitiveComponent Object Reference") (OtherActor :type "Actor Object Reference") (OtherComp :type "PrimitiveComponent Object Reference") (OtherBodyIndex :type Integer) (bFromSweep :type Boolean) (SweepResult :type "HitResult Structure (by ref)"))
  ;[1 1 1] プレイヤーと衝突処理
  (if (`ActorComponent.ComponentHasTag` OtherComp "Player")
    (bind _returnvalue (`self.SetupPlayerUse` (`self.K2_GetActorLocation` (`GameplayStatics.GetPlayerPawn` 0)) (`self.Sphere1`)))
    (if _returnvalue
      (`SoundManagerBase.PlaySound2D` "/Game/Main/Sound/SE/GetMagatama/GetMagatama_Cue.GetMagatama_Cue" "SE" 1.0 1.0 0.0 null null)
      (`/Game/Main/BP/MiniMap/BP_MiniMapActor.SetHidden` (`self.MiniMapManager`) (`ChildActorComponent.ChildActor` (`self.MiniMapRenderActor`)))
      (bind _asbp_magatama_bit (cast `/Game/Main/BP/Magatama/BP_MagatamaBit` (`ChildActorComponent.ChildActor` (`self.BP_MagatamaBit`))))
      (set `/Game/Main/BP/Magatama/BP_MagatamaBit.Move` true _asbp_magatama_bit)
      (`self.SetEffectActive` false))))

(event `self.ReceiveTick`
  (params (DeltaSeconds :type "Float (single-precision)"))
  (bind _playerbp (`self.PlayerBP`))
  ;[1 1 1] 更新処理
  (`self.Update` _playerbp (`self.Sphere1`))
  (set `self.speedRate` (`/Game/Main/BP/Player/BP_Player.Speedrate` _playerbp))
  (set `self.OldHitFlg` (`self.HitFlg`))
  (set `self.HitFlg` false))

(event `self.Sphere1.OnComponentHit`
  (params (HitComponent :type "PrimitiveComponent Object Reference") (OtherActor :type "Actor Object Reference") (OtherComp :type "PrimitiveComponent Object Reference") (NormalImpulse :type "Vector Structure") (Hit :type "HitResult Structure (by ref)"))
  ;[1 1 1] 敵へのダメージ処理
  (if (`self.ActorHasTag` OtherActor "Enemy")
    (bind _output_get (set `self.HitFlg` true))
    (bind _returnvalue (and _output_get (not (`self.OldHitFlg`))))
    (if _returnvalue
      (bind _asbp_enemy_base (cast `/Game/Main/BP/Enemy/EnemyBase/BP_EnemyBase` OtherActor)
        (:`then`
          (`/Game/Main/BP/Enemy/EnemyBase/BP_EnemyBase.HitPlayerAttack` _asbp_enemy_base (`KismetMathLibrary.Normal` (`self.GetNockBackForce`)) (`self.GetDamage`))
          (`SoundManagerBase.PlaySound2D` "/Game/Main/Sound/SE/AttackMagatama/AttackMagatama_Cue.AttackMagatama_Cue" "SE" 1.0 1.0 0.0 null null))
        (:`CastFailed`
          _))
      (bind _returnvalue_2 (`self.ResetWait` _returnvalue :!label _label))
      (if _returnvalue_2
        (`/Game/Main/BP/MiniMap/BP_MiniMapActor.SetUnHidden` (`self.MiniMapManager`) (`ChildActorComponent.ChildActor` (`self.MiniMapRenderActor`)))
        (bind _asbp_magatama_bit (cast `/Game/Main/BP/Magatama/BP_MagatamaBit` (`ChildActorComponent.ChildActor` (`self.BP_MagatamaBit`))))
        (set `/Game/Main/BP/Magatama/BP_MagatamaBit.Move` false _asbp_magatama_bit)
        (`self.SetEffectActive` true)))
    (else
      (goto _label))))

(event `self.ReceiveBeginPlay`
  (bind _returnvalue (`GameplayStatics.GetActorOfClass` "/Game/Main/BP/MiniMap/BP_MiniMapActor.BP_MiniMapActor_C"))
  (set `self.MiniMapManager` _returnvalue)
  (bind _asbp_player (cast `/Game/Main/BP/Player/BP_Player` (`GameplayStatics.GetPlayerPawn` 0)))
  (set `self.PlayerBP` _asbp_player))

(event `self.ReceiveHit`
  (params (MyComp :type "PrimitiveComponent Object Reference") (Other :type "Actor Object Reference") (OtherComp :type "PrimitiveComponent Object Reference") (bSelfMoved :type Boolean) (HitLocation :type "Vector Structure") (HitNormal :type "Vector Structure") (NormalImpulse :type "Vector Structure") (Hit :type "HitResult Structure (by ref)"))
  (if (`self.GetHitEffect`)
    (`GameplayStatics.SpawnEmitterAtLocation` "/Game/Main/Effect/Enemy/P_MagatamaHitSpark.P_MagatamaHitSpark" HitLocation)))

(event `self.SettingFiled`
  (params (filed :type "E_FiledState Enum" :default "Normal"))
  (bind (_value _returnvalue) (`BlueprintMapLibrary.Map_Find` (`self.FiledPSEffect`) filed))
  (bind (_value_2 _returnvalue_2) (`BlueprintMapLibrary.Map_Find` (`self.FiledNSEffect`) filed))
  (if _returnvalue_2
    (bind _returnvalue_3 (`NiagaraFunctionLibrary.SpawnSystemAttached` _value_2 (`self.Sphere1`) "None" (0.0 0.0 0.0) (struct) "KeepRelativeOffset"))
    (bind _output_get (set `self.NS` _returnvalue_3))
    (`SceneComponent.SetHiddenInGame` _output_get true false)
    (`SceneComponent.SetHiddenInGame` (`self.NS_MagatamaAura`) false false)
    (elif _returnvalue
      (bind _returnvalue_4 (`GameplayStatics.SpawnEmitterAttached` _value (`self.Sphere1`)))
      (bind _output_get_2 (set `self.PS` _returnvalue_4))
      (`SceneComponent.SetHiddenInGame` _output_get_2 true false)
      (`SceneComponent.SetHiddenInGame` (`self.NS_MagatamaAura`) false false))))

(event `SetEffectActive`
  (params (NewHidden :type Boolean))
  (bind _ns (`self.NS`))
  (bind _ps (`self.PS`))
  (`/Engine/EditorBlueprintResources/StandardMacros.IsValid` _ns
    (:`Is Valid`
      (`SceneComponent.SetHiddenInGame` _ns NewHidden false))
    (:`Is Not Valid`
      (`/Engine/EditorBlueprintResources/StandardMacros.IsValid` _ps
        (:`Is Valid`
          (`SceneComponent.SetHiddenInGame` _ps NewHidden false))))))

(fn `UserConstructionScript`)