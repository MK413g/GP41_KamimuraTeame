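; BP_SpawnThunder is a spawner actor that repeatedly creates BP_Lightning at random positions until the game ends.
; On Tick, a DoOnce and Delay pair forms a repeating timer using the Time variable.
; Each location scales a sine/cosine vector by a random distance up to Range, around the world origin at zero height.
; Sine and cosine take separate random angles, so the spread is not strictly circular.
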(event `self.ReceiveTick`
  (params (DeltaSeconds :type "Float (single-precision)"))
  (bind _returnvalue (`KismetMathLibrary.RandomFloatInRange` 0.0 360.0))
  (if (not (`MainGameEndManager.GetGameEnd`))
    (`/Engine/EditorBlueprintResources/StandardMacros.DoOnce` false :!label _label
      (:`Completed`
        (`KismetSystemLibrary.Delay` (`self.Time`))
        (`|SpawnActorFromClass` "/Game/Main/BP/Player/BP_Lightning.BP_Lightning_C" (`KismetMathLibrary.MakeTransform` (* (`KismetMathLibrary.MakeVector` (`KismetMathLibrary.DegSin` _returnvalue) (`KismetMathLibrary.DegCos` _returnvalue)) (`KismetMathLibrary.RandomFloatInRange` 0.0 (`self.Range`)))) "Undefined" "OverrideRootScale" null null)
        (goto _label :!via `Reset`)))))

(fn `UserConstructionScript`)