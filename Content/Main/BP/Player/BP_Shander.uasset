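; BP_Shander is a lightning pulse actor that can stun players for a short time, then destroys itself.
; A Wave timeline drives the pulse material's Time parameter and the child actor's XY scale, destroying the actor when finished.
; Outside overlaps stun the player while Hitflg is set, and an Inside overlap clears that flag.
; The Construction Script applies the same material and scale from a Time variable, allowing an editor preview.
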(event `self.ReceiveBeginPlay`
  (bind _returnvalue (`PrimitiveComponent.CreateDynamicMaterialInstance` (`self.StaticMesh`) 0 "/Game/LevelDesign/Effects/Material/M_LightningPulse_Inst.M_LightningPulse_Inst" "None"))
  (bind (_direction `_新規track_0`) (`Timeline|wave`)
    (:`Update`
      (`MaterialInstanceDynamic.SetScalarParameterValue` _returnvalue "Time" `_新規track_0`)
      (bind _returnvalue_2 (+ (* `_新規track_0` (`self.scalerate`)) (`self.scale`)))
      (`SceneComponent.SetRelativeScale3D` (`self.ChildActor`) (`KismetMathLibrary.MakeVector` _returnvalue_2 _returnvalue_2 1.0)))
    (:`Finished`
      (`self.K2_DestroyActor`))))

(event `self.inside.OnComponentBeginOverlap`
  (params (OverlappedComponent :type "PrimitiveComponent Object Reference") (OtherActor :type "Actor Object Reference") (OtherComp :type "PrimitiveComponent Object Reference") (OtherBodyIndex :type Integer) (bFromSweep :type Boolean) (SweepResult :type "HitResult Structure (by ref)"))
  (if (`self.ActorHasTag` OtherActor "Player")
    (set `self.hitflg` false)))

(event `self.outside.OnComponentBeginOverlap`
  (params (OverlappedComponent :type "PrimitiveComponent Object Reference") (OtherActor :type "Actor Object Reference") (OtherComp :type "PrimitiveComponent Object Reference") (OtherBodyIndex :type Integer) (bFromSweep :type Boolean) (SweepResult :type "HitResult Structure (by ref)"))
  (if (`self.ActorHasTag` OtherActor "Player")
    (if (`self.hitflg`)
      (bind _asbp_player (cast `/Game/Main/BP/Player/BP_Player` OtherActor))
      (`PlayerBase.SetStun` _asbp_player 2.0))))

(fn `UserConstructionScript`
  (bind _time (`self.time`))
  (bind _returnvalue (+ (* _time (`self.scalerate`)) (`self.scale`)))
  (bind _returnvalue_2 (`PrimitiveComponent.CreateDynamicMaterialInstance` (`self.StaticMesh`) 0 "/Game/LevelDesign/Effects/Material/M_LightningPulse_Inst.M_LightningPulse_Inst" "None"))
  (`MaterialInstanceDynamic.SetScalarParameterValue` _returnvalue_2 "Time" _time)
  (`SceneComponent.SetRelativeScale3D` (`self.ChildActor`) (`KismetMathLibrary.MakeVector` _returnvalue _returnvalue 1.0)))