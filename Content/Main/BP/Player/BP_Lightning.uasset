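; BP_Lightning is a one-shot spawner actor that creates a lightning strike at its own transform.
; CreateLightning spawns BP_ky_lightning1, waits briefly, spawns BP_Shander at the same location and rotation, then destroys the spawner.
; BP_Shander's X and Y scale are multiplied by the Scale variable, while Z stays fixed at one.
; A Q key press bound in the actor also calls CreateLightning.
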(event `CreateLightning`
  (bind (_returnvalue_location _returnvalue_rotation _returnvalue_scale) (`KismetMathLibrary.BreakTransform` (`self.GetTransform`)))
  (bind (_returnvalue_x _returnvalue_y) (`KismetMathLibrary.BreakVector` (* _returnvalue_scale (`self.scale`))))
  (`|SpawnActorFromClass` "/Game/LevelDesign/Effects/Blueprint/BP_ky_lightning1.BP_ky_lightning1_C" (`self.GetTransform`) "Undefined" "OverrideRootScale" null null)
  (`KismetSystemLibrary.Delay` 0.4)
  (`|SpawnActorFromClass` "/Game/Main/BP/Player/BP_Shander.BP_Shander_C" (`KismetMathLibrary.MakeTransform` _returnvalue_location _returnvalue_rotation (`KismetMathLibrary.MakeVector` _returnvalue_x _returnvalue_y 1.0)) "Undefined" "OverrideRootScale" null null)
  (`self.K2_DestroyActor`))

(event `self.ReceiveBeginPlay`)

(event `Key|Q` :consume false
  (params (Key :type "Key Structure"))
  (:`Pressed`
    (`self.CreateLightning`)))

(fn `UserConstructionScript`)