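; BP_pool is a pool actor that slows the player while they overlap its Plane component.
; On begin overlap, it caches the BP_Player's MoveSpeed and sets the character's max walk speed to two-thirds of it.
; On end overlap, it restores the cached speed.
; Both events filter by the Player tag and cast, but apply the change to player character 0.
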(event `self.Plane.OnComponentBeginOverlap`
  (params (OverlappedComponent :type "PrimitiveComponent Object Reference") (OtherActor :type "Actor Object Reference") (OtherComp :type "PrimitiveComponent Object Reference") (OtherBodyIndex :type Integer) (bFromSweep :type Boolean) (SweepResult :type "HitResult Structure (by ref)"))
  (if (`self.ActorHasTag` OtherActor "Player")
    (bind _asbp_player (cast `/Game/Main/BP/Player/BP_Player` OtherActor))
    (bind _output_get (set `self.movespeed` (`PlayerBase.MoveSpeed` _asbp_player)))
    (set `CharacterMovementComponent.MaxWalkSpeed` (* (/ _output_get 3.0) 2.0) (`Character.CharacterMovement` (`GameplayStatics.GetPlayerCharacter` 0)))))

(event `self.Plane.OnComponentEndOverlap`
  (params (OverlappedComponent :type "PrimitiveComponent Object Reference") (OtherActor :type "Actor Object Reference") (OtherComp :type "PrimitiveComponent Object Reference") (OtherBodyIndex :type Integer))
  (if (`self.ActorHasTag` OtherActor "Player")
    (cast `/Game/Main/BP/Player/BP_Player` OtherActor)
    (set `CharacterMovementComponent.MaxWalkSpeed` (`self.movespeed`) (`Character.CharacterMovement` (`GameplayStatics.GetPlayerCharacter` 0)))))

(fn `UserConstructionScript`)