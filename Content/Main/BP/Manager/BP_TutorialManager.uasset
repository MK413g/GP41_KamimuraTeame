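; BP_TutorialManager runs the tutorial stage: on play it creates the Tutorial widget at the FirstWait step, starts the minimap and plays the stage BGM.
; Update events advance the widget's text and, at the CollectMagatama step, spawn a magatama creator actor and restart the minimap.
; Jump advances text when the widget accepts input.
; Overridden getters expose widget progress flags, and SoundFade fades out the music.
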(event `self.ReceiveBeginPlay`
  (bind _returnvalue (`|CreateWidget` "/Game/Main/BP/Widget/Tutorial.Tutorial_C"))
  (bind _output_get (set `self.widget` _returnvalue))
  (`UserWidget.AddToViewport` _output_get 0)
  (set `/Game/Main/BP/Widget/Tutorial.Owner` self _output_get)
  (`/Game/Main/BP/Widget/Tutorial.NextText` _output_get "FirstWait")
  (bind _returnvalue_2 (`GameplayStatics.GetActorOfClass` "/Game/Main/BP/MiniMap/BP_MiniMapActor.BP_MiniMapActor_C"))
  (`/Game/Main/BP/MiniMap/BP_MiniMapActor.Start` _returnvalue_2)
  (bind _returnvalue_3 (`GameplayStatics.SpawnSound2D` "/Game/Main/Sound/BGM/Stage/StageBGM_1.StageBGM_1" 1.0 1.0 0.0 null))
  (set `self.SoundBGM` _returnvalue_3))

(event `self.UpdateWidget`
  (params (nexttype :type "E_TutorialType Enum" :default "FirstWait"))
  (`/Game/Main/BP/Widget/Tutorial.NextText` (`self.widget`) nexttype))

(event `InputAction|Jump` :consume false
  (params (Key :type "Key Structure"))
  (bind _widget (`self.widget`))
  (:`Pressed`
    (if (`/Game/Main/BP/Widget/Tutorial.InputNextTextKey` _widget)
      (`/Game/Main/BP/Widget/Tutorial.NextTextArray` _widget))))

(event `self.UpdateTutorial`
  (if (`|EnumEquality` (`self.GetTutorialType`) "CollectMagatama")
    (`|SpawnActorFromClass` "/Game/Main/BP/Tutorial/BP_CreateMagatamaActor.BP_CreateMagatamaActor_C" (`KismetMathLibrary.MakeTransform` (0.0 0.0 0.0)) "Undefined" "OverrideRootScale" null null)
    (bind _returnvalue (`GameplayStatics.GetActorOfClass` "/Game/Main/BP/MiniMap/BP_MiniMapActor.BP_MiniMapActor_C"))
    (`/Game/Main/BP/MiniMap/BP_MiniMapActor.Start` _returnvalue)))

(event `SoundFade`
  (bind _soundbgm (`self.SoundBGM`))
  (`/Engine/EditorBlueprintResources/StandardMacros.IsValid` _soundbgm
    (:`Is Valid`
      (`AudioComponent.FadeOut` _soundbgm 1.5 0.0 "Linear"))))

(fn `GetExplanation`
  (returns (ReturnValue :type Boolean))
  (bind _widget (`self.widget`))
  (`parent.GetExplanation`)
  (`/Engine/EditorBlueprintResources/StandardMacros.IsValid` _widget
    (:`Is Valid`
      (return (`/Game/Main/BP/Widget/Tutorial.ExplanationFlg` _widget)))))

(fn `GetInputTextTutorial`
  (returns (ReturnValue :type Boolean))
  (`parent.GetInputTextTutorial`)
  (return (`/Game/Main/BP/Widget/Tutorial.InputNextTextKey` (`self.widget`))))

(fn `GetNext`
  (returns (ReturnValue :type Boolean))
  (bind _widget (`self.widget`))
  (`parent.GetNext`)
  (`/Engine/EditorBlueprintResources/StandardMacros.IsValid` _widget
    (:`Is Valid`
      (return (`/Game/Main/BP/Widget/Tutorial.next` _widget)))))

(fn `GetNextTutorial`
  (returns (ReturnValue :type Boolean))
  (`parent.GetNextTutorial`)
  (return (`/Game/Main/BP/Widget/Tutorial.NextFlg` (`self.widget`))))

(fn `UserConstructionScript`)