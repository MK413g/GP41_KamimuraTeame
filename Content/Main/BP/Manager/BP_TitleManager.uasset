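; Title screen manager that creates and shows the Title widget on BeginPlay and sets the game instance's stage state to Title.
; The MoveForward axis cycles a two-option selection with wraparound and pushes it to the widget, using an axis threshold and a DoOnce reset by a short Delay to throttle held input.
; Pressing Jump passes the current selection to the widget's Decision function.
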(event `InputAction|Jump`
  (params (Key :type "Key Structure"))
  (:`Pressed`
    (`/Game/Main/BP/Widget/Title.Decision` (`self.TitleWidget`) (`self.SelectNumber`))))

(event `InputAxis|MoveForward` :consume false
  (params (AxisValue :type "Float (single-precision)"))
  (if (>= (`KismetMathLibrary.Abs` AxisValue) 0.6)
    (`|ExecutionSequence`
      (:`then_0`
        (`/Engine/EditorBlueprintResources/StandardMacros.DoOnce` false :!label _label
          (:`Completed`
            (if (> AxisValue 0.0)
              (set `self.SelectNumber` (- (`self.SelectNumber`) 1))
              (if (< (`self.SelectNumber`) 0)
                (set `self.SelectNumber` 1))
              (else
                (set `self.SelectNumber` (+ (`self.SelectNumber`) 1))
                (if (> (`self.SelectNumber`) 1)
                  (set `self.SelectNumber` 0))))
            (`/Game/Main/BP/Widget/Title.SetSelect` (`self.TitleWidget`) (`self.SelectNumber`)))))
      (:`then_1`
        (`KismetSystemLibrary.Delay` 0.2)
        (goto _label :!via `Reset`)))))

(event `self.ReceiveBeginPlay`
  (bind _returnvalue (`|CreateWidget` "/Game/Main/BP/Widget/Title.Title_C"))
  (bind _output_get (set `self.TitleWidget` _returnvalue))
  (`UserWidget.AddToViewport` _output_get 0)
  (`GameStageInstance.SetStageState` (`GameStageInstance.GetInstance`) "Title"))

(fn `UserConstructionScript`)