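; Main-level end manager that handles game clear and game over, extending a parent manager whose state it polls on Tick.
; Clear triggers slow motion, stops the player, removes Magatama, hides the night sublevel and plays a Sequencer cutscene through tagged cine cameras.
; The GameOver widget appears immediately on game over or via a sequencer-called event on clear, with a variant for Stage5.
; Debounced axis input cycles its options and Jump confirms, opening Level01 or Title.
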(event `Key|End`
  (params (Key :type "Key Structure"))
  (:`Pressed`
    (`parent.ReceiveBeginPlay` :!label _label)
    (bind _outactors (`GameplayStatics.GetAllActorsOfClassWithTag` "/Script/CinematicCamera.CineCameraActor" "Enemycamera"))
    (for _array_element _outactors
      (set `self.EnemyCamera` _array_element))
    (bind _outactors_2 (`GameplayStatics.GetAllActorsOfClassWithTag` "/Script/CinematicCamera.CineCameraActor" "EndCamera"))
    (for _array_element_2 _outactors_2
      (set `self.Camera` _array_element_2))))

(event `self.ReceiveBeginPlay`
  (goto _label))

(event `self.ReceiveEndPlay`
  (params (EndPlayReason :type "EEndPlayReason Enum" :default "Destroyed"))
  (goto _label))

(event `self.ReceiveTick`
  (params (DeltaSeconds :type "Float (single-precision)"))
  (`self.ExecEnumOutput` (`self.GetStat`)
    (:`Clear`
      (`self.SetClearStat`))
    (:`Over`
      (`self.SetOverStat`))))

(event `SetWidget`
  ;[1 1 1] シーケンサーで呼び出しイベント
  (bind _returnvalue (`|CreateWidget` "/Game/Main/BP/Widget/GameOver.GameOver_C"))
  (bind _output_get (set `self.GameEndWidget` _returnvalue))
  (`UserWidget.AddToViewport` _output_get 0)
  (if (`|EnumEquality` (`GameStageInstance.GetLevelState` (`GameStageInstance.GetInstance`)) "Stage5")
    (`/Game/Main/BP/Widget/GameOver.SetGameClearEnd` _output_get)
    (else
      (`/Game/Main/BP/Widget/GameOver.SetGameClear` _output_get))))

(event `GameClearAnimStop`
  ;[1 1 1] シーケンサーで呼び出しイベント
  (`MovieSceneSequencePlayer.Pause` (`self.GameClearSequence`)))

(event `InputAxis|MoveForward` :consume false
  (params (AxisValue :type "Float (single-precision)"))
  (bind _gameendwidget (`self.GameEndWidget`))
  ;[1 1 1] 選択処理
  (if (> (`KismetMathLibrary.Abs` AxisValue) 0.6)
    (`|ExecutionSequence`
      (:`then_0`
        (`/Engine/EditorBlueprintResources/StandardMacros.DoOnce` false :!label _label_2
          (:`Completed`
            (`/Engine/EditorBlueprintResources/StandardMacros.IsValid` _gameendwidget
              (:`Is Valid`
                (if (and (`/Game/Main/BP/Widget/GameOver.input` _gameendwidget) (`self.Inputend`))
                  (if (> AxisValue 0.0)
                    (set `self.widegtinputNumber` (- (`self.widegtinputNumber`) 1))
                    (else
                      (set `self.widegtinputNumber` (+ (`self.widegtinputNumber`) 1))))
                  (if (> (`self.widegtinputNumber`) 2)
                    (set `self.widegtinputNumber` 0)
                    (elif (< (`self.widegtinputNumber`) 0)
                      (set `self.widegtinputNumber` 2)))
                  (`/Game/Main/BP/Widget/GameOver.InputSetting` (`self.GameEndWidget`) (`self.widegtinputNumber`))))))))
      (:`then_1`
        (`KismetSystemLibrary.Delay` 0.2)
        (goto _label_2 :!via `Reset`)))))

(event `InputAction|Jump` :consume false
  (params (Key :type "Key Structure"))
  (bind _gameendwidget (`self.GameEndWidget`))
  (:`Pressed`
    ;[1 1 1] 決定処理
    (`/Engine/EditorBlueprintResources/StandardMacros.IsValid` _gameendwidget
      (:`Is Valid`
        (if (`self.Inputend`)
          (if (`/Game/Main/BP/Widget/GameOver.input` _gameendwidget)
            (`/Engine/EditorBlueprintResources/StandardMacros.DoOnce` false :!label _label_3
              (:`Completed`
                (bind _returnvalue (`GameStageInstance.SetNextStage` (`GameStageInstance.GetInstance`)))
                (if _returnvalue
                  (set `self.Inputend` false :!label _label_4)
                  (`SoundManagerBase.PlaySound2D` "/Game/Main/Sound/SE/Decision/Decision_Cue.Decision_Cue" "SE" 1.0 1.0 0.0 null null)
                  (`KismetSystemLibrary.Delay` 1.0)
                  (`GameplayStatics.OpenLevelBySoftObjectPtr` "/Game/Main/Level/Title.Title")
                  (elif (== (`self.widegtinputNumber`) 0)
                    (set `self.Inputend` false)
                    (`SoundManagerBase.PlaySound2D` "/Game/Main/Sound/SE/Decision/Decision_Cue.Decision_Cue" "SE" 1.0 1.0 0.0 null null)
                    (`KismetSystemLibrary.Delay` 0.2)
                    (`GameplayStatics.OpenLevelBySoftObjectPtr` "/Game/LevelDesign/Levels/Level01.Level01")
                    (elif (== (`self.widegtinputNumber`) 2)
                      (goto _label_4)
                      (else
                        (goto _label_3 :!via `Reset`)))))))
            (elif (`/Game/Main/BP/Widget/GameOver.end` _gameendwidget)
              (goto _label_4))))))))

(event `self.SetClearStat`
  (bind _enemy (`self.enemy`))
  (`parent.SetClearStat`)
  (`/Engine/EditorBlueprintResources/StandardMacros.DoOnce` false
    (:`Completed`
      (`/Game/Main/BP/Player/SlowMacroLibrary.SetSlow` 0.1 0.15)
      (`KismetSystemLibrary.Delay` 0.3)
      (`self.K2_SetActorLocation` (`self.EnemyCamera`) (+ (+ (* (`KismetMathLibrary.Normal` (`KismetMathLibrary.GetForwardVector` (`KismetMathLibrary.MakeRotator` 0.0 0.0 (.yaw (`self.K2_GetActorRotation` _enemy))))) 1000.0) (`self.Offset`)) (`self.K2_GetActorLocation` _enemy)) false false)
      (bind _asbp_player (cast `/Game/Main/BP/Player/BP_Player` (`GameplayStatics.GetPlayerPawn` 0)))
      (`/Game/Main/BP/Player/BP_Player.PlayerStop` _asbp_player)
      (`/Game/Main/BP/Enemy/EnemyBase/BP_EnemyBase.NoShowWidget` (`self.enemy`))
      (bind _outactors (`GameplayStatics.GetAllActorsOfClass` "/Game/Main/BP/Magatama/BP_Magatama.BP_Magatama_C"))
      (for _array_element _outactors
        (`self.K2_DestroyActor` _array_element))
      (`PlayerController.SetViewTargetWithBlend` (`GameplayStatics.GetPlayerController` 0) (`self.Camera`) 1e-05 "VTBlend_Linear" 0.0 true)
      (bind _returnvalue (`GameplayStatics.GetActorOfClass` "/Game/Main/BP/Manager/SubLevel/BP_TestSubLevel.BP_TestSubLevel_C"))
      (`/Game/Main/BP/Manager/SubLevel/BP_TestSubLevel.NoShowSubLevel` _returnvalue "Night")
      (bind (_outactor _returnvalue_2) (`LevelSequencePlayer.CreateLevelSequencePlayer` "/Game/Main/Sequence/GameClearSequence/GameClearSequence.GameClearSequence"))
      (bind _output_get (set `self.GameClearSequence` _returnvalue_2))
      (`MovieSceneSequencePlayer.Play` _output_get))))

(event `self.SetOverStat`
  (`parent.SetOverStat`)
  (bind _returnvalue (`|CreateWidget` "/Game/Main/BP/Widget/GameOver.GameOver_C"))
  (bind _output_get (set `self.GameEndWidget` _returnvalue))
  (`UserWidget.AddToViewport` _output_get 0)
  (`/Game/Main/BP/Widget/GameOver.SetGaemOverEvent` _output_get)
  (set `self.GameOver` true))

(fn `GetSequence`
  (returns (GameClearSequence :type "LevelSequencePlayer Object Reference"))
  (return (`self.GameClearSequence`)))

(fn `UserConstructionScript`)