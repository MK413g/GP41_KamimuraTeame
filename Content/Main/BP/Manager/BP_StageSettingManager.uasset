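; Stage setup manager that configures the player, enemy and level for the current stage on BeginPlay.
; It reads a stage state from a data table, which selects the player's data table name and the sublevel to load.
; After spawning the enemy, it aims tagged cine cameras at it, hands it to the minimap renderer and end manager, starts the minimap, then loads the sublevel.
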(event `self.ReceiveBeginPlay`
  (`parent.ReceiveBeginPlay`)
  (`self.GetDataTableState`) ; データテーブルから値を取得
  (bind _asbp_player (cast `/Game/Main/BP/Player/BP_Player` (`GameplayStatics.GetPlayerPawn` 0)))
  (set `PlayerBase.LoadDataName` (`BlueprintMapLibrary.Map_Find` (`self.PlayerFiledName`) (`self.BreakFiled` (`self.state`))) _asbp_player)
  (`PlayerBase.SetDataTable` _asbp_player) ; プレイヤーのデータテーブルを取得
  ;[1 1 1] 敵を生成
  (bind _returnvalue (`self.CreateEnemy`))
  (`/Engine/EditorBlueprintResources/StandardMacros.IsValid` _returnvalue
    (:`Is Valid`
      (bind _outactors (`GameplayStatics.GetAllActorsOfClassWithTag` "/Script/CinematicCamera.CineCameraActor" "Enemycamera"))
      (for _array_element _outactors
        (set `CineCameraActor.LookatTrackingSettings` (make `CameraLookatTrackingSettings` true false 0.0 (`|ConvertAsset` _returnvalue)) _array_element))
      (bind _returnvalue_2 (`GameplayStatics.GetActorOfClass` "/Game/Main/BP/MiniMap/BP_MiniMapRenderActor.BP_MiniMapRenderActor_C"))
      (set `/Game/Main/BP/MiniMap/BP_MiniMapRenderActor.TargetActor` _returnvalue _returnvalue_2)
      (bind _returnvalue_3 (`GameplayStatics.GetActorOfClass` "/Game/Main/BP/Manager/BP_MainEndManager.BP_MainEndManager_C"))
      (bind _asbp_enemy_base (cast `/Game/Main/BP/Enemy/EnemyBase/BP_EnemyBase` _returnvalue))
      (set `/Game/Main/BP/Manager/BP_MainEndManager.enemy` _asbp_enemy_base _returnvalue_3)
      (bind _returnvalue_4 (`GameplayStatics.GetActorOfClass` "/Game/Main/BP/MiniMap/BP_MiniMapActor.BP_MiniMapActor_C"))
      (`/Game/Main/BP/MiniMap/BP_MiniMapActor.Start` _returnvalue_4)
      (bind _returnvalue_5 (`GameplayStatics.GetActorOfClass` "/Game/Main/BP/Manager/SubLevel/BP_TestSubLevel.BP_TestSubLevel_C"))
      (`/Game/Main/BP/Manager/SubLevel/BP_TestSubLevel.LoadLevel` _returnvalue_5 (`self.BreakFiled` (`self.state`))))))

(fn `UserConstructionScript`)