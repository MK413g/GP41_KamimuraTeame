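; Snake enemy that chases the player, performs rush attacks and fires poison bullets, with stats loaded from DT_SnakeStatus at BeginPlay.
; Attack functions are timer-driven state steps using SecCnt and flags: face the player, attack, recover.
; FinAction resets that state and asks BP_SnakeAI to select the next action.
; Mesh hits damage the player while ATK is positive, and death fades material opacity and aura before destroying both components.
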(event `self.ReceiveBeginPlay`
  (bind _pt_enemyaura (`self.PT_EnemyAura`))
  (`|ExecutionSequence`
    (:`then_0`
      (`FXSystemComponent.SetActorParameter` _pt_enemyaura "VertSurfaceActor" self)
      (`SceneComponent.SetRelativeScale3D` _pt_enemyaura (0.033333 1.0 1.0))
      (`FXSystemComponent.SetFloatParameter` _pt_enemyaura "SpawnRate" 0.0))
    (:`then_1`
      (`self.FinAction`)
      (bind _returnvalue (`|GetDataTableRow` "/Game/Main/DataTable/DT_SnakeStatus.DT_SnakeStatus" "SnakeState")
        (:`then`
          (set `self.HP` (break `/Game/Main/BP/Enemy/Snake/ST_SnakeStatus` _returnvalue))
          (set `self.MoveSpeed_Sec` (`.MoveSpeed_38_D2B7BE2D4875D1C1D3BB479A2B5DA3E0` (break `/Game/Main/BP/Enemy/Snake/ST_SnakeStatus` _returnvalue)))
          (set `self.RotateSpeed_Sec` (`.RotateSpeed_37_3CB5073D49250B92406A308753F0C366` (break `/Game/Main/BP/Enemy/Snake/ST_SnakeStatus` _returnvalue)))
          (set `self.RushSpeed` (`.RushSpeed_36_0739916243CFA30A1E13DAA08C76ECE9` (break `/Game/Main/BP/Enemy/Snake/ST_SnakeStatus` _returnvalue)))
          (set `self.RushPrepareSec` (`.RushPrepareSec_18_16776D5645EAB20195AB3BB6786874AD` (break `/Game/Main/BP/Enemy/Snake/ST_SnakeStatus` _returnvalue)))
          (set `self.RushSec` (`.RushSec_11_AB02E68548097F459979089B3829EDCE` (break `/Game/Main/BP/Enemy/Snake/ST_SnakeStatus` _returnvalue)))
          (set `self.RushAfterSec` (`.AfterRushSec_17_7BBDDE1147BF97109E0DA0BB10737B88` (break `/Game/Main/BP/Enemy/Snake/ST_SnakeStatus` _returnvalue)))
          (set `self.RushAttackNum` (`.RushAttackNum_19_BC100696497CE9C4D28956A2CAC31D15` (break `/Game/Main/BP/Enemy/Snake/ST_SnakeStatus` _returnvalue)))
          (set `self.PoisonBulletPrepareSec` (`.PoisonBulletPrepareSec_59_B4D154714D4A676881844B932A02697E` (break `/Game/Main/BP/Enemy/Snake/ST_SnakeStatus` _returnvalue)))
          (set `self.AfterShotPoisonSec` (`.AfterPoisonBulletShotSec_58_9132FF5643AC4B5C9B5E35A537AC9DF9` (break `/Game/Main/BP/Enemy/Snake/ST_SnakeStatus` _returnvalue)))
          (set `self.PoisonBulletAttackNum` (`.PoisonBulletAttackNum_57_DFAE1E66452F11444087469E4F98AD59` (break `/Game/Main/BP/Enemy/Snake/ST_SnakeStatus` _returnvalue)))
          (set `self.PoisonBulletSpeedNum` (`.PoisonBulletSpeed_56_5AC1BC134359E19FAF3D19BE0D0C736E` (break `/Game/Main/BP/Enemy/Snake/ST_SnakeStatus` _returnvalue)))
          (set `self.PoisonBulletLifeSec` (`.PoisonBulletLifeSec_55_6812D13142422F0CF871EEB2611C0673` (break `/Game/Main/BP/Enemy/Snake/ST_SnakeStatus` _returnvalue)))
          (`parent.ReceiveBeginPlay`))))))

(event `self.ReceiveTick`
  (params (DeltaSeconds :type "Float (single-precision)"))
  (`parent.ReceiveTick` DeltaSeconds))

(event `self.snake_model.OnComponentHit`
  (params (HitComponent :type "PrimitiveComponent Object Reference") (OtherActor :type "Actor Object Reference") (OtherComp :type "PrimitiveComponent Object Reference") (NormalImpulse :type "Vector Structure") (Hit :type "HitResult Structure (by ref)"))
  (bind _atk (`self.ATK`))
  (if (`self.ActorHasTag` OtherActor "Player")
    (bind _asbp_player (cast `/Game/Main/BP/Player/BP_Player` OtherActor))
    (if (> _atk 0.0)
      (`PlayerBase.SetDamage` _asbp_player _atk (0.0 0.0 0.0) 0.0))))

(fn `FinAction`
  (bind _asbp_snake_ai (cast `/Game/Main/BP/Enemy/Snake/BP_SnakeAI` (`AIBlueprintHelperLibrary.GetAIController` self)))
  (`/Game/Main/BP/Enemy/Snake/BP_SnakeAI.SelectAction` _asbp_snake_ai)
  (set `self.AttackStartedFlag` false)
  (set `self.FinActionFlag` false)
  (set `self.TimeCnt` 0.0))

(fn `MoveToPlayerSnake`
  (if (`self.FinActionFlag`)
    (`self.FinAction`)
    (else
      (`self.MoveToPlayer`))))

(fn `ShotPoisonBullet`
  (bind (_returnvalue_location _returnvalue_rotation) (`KismetMathLibrary.BreakTransform` (`self.GetTransform`)))
  (if (`self.AttackStartedFlag`)
    (bind _fin (`self.SecCnt` (`self.AfterShotPoisonSec`)))
    (if _fin
      (`self.FinAction`))
    (else
      (`self.Rotate To Face Player XY plane`)
      (bind _fin_2 (`self.SecCnt` (`self.PoisonBulletPrepareSec`)))
      (if _fin_2
        (bind _returnvalue (`|SpawnActorFromClass` "/Game/Main/BP/Enemy/BP_PoisonBullet.BP_PoisonBullet_C" (`KismetMathLibrary.ComposeTransforms` (`KismetMathLibrary.Conv_VectorToTransform` (`self.PoisonBulletSpawnPos`)) (`KismetMathLibrary.MakeTransform` _returnvalue_location _returnvalue_rotation)) "Undefined" "OverrideRootScale" null null))
        (set `/Game/Main/BP/Enemy/BP_PoisonBullet.ATK` (`self.PoisonBulletAttackNum`) _returnvalue)
        (set `/Game/Main/BP/Enemy/BP_PoisonBullet.MoveVec` (`self.GetActorForwardVector`) _returnvalue)
        (set `/Game/Main/BP/Enemy/BP_PoisonBullet.Speed` (`self.PoisonBulletSpeedNum`) _returnvalue)
        (set `/Game/Main/BP/Enemy/BP_PoisonBullet.LifeSec` (`self.PoisonBulletLifeSec`) _returnvalue)
        (set `self.AttackStartedFlag` true)
        (set `self.FinActionFlag` true)))))

(fn `SnakeDead`
  (bind (_fin _nowsec) (`self.SecCnt` (`self.DeadDirectingSec`)))
  (if _fin
    (`ActorComponent.K2_DestroyComponent` (`self.snake_model`))
    (`ActorComponent.K2_DestroyComponent` (`self.PT_EnemyAura`))
    (else
      (bind _returnvalue (`PrimitiveComponent.CreateDynamicMaterialInstance` (`self.snake_model`) 0 "/Game/Main/Meshes/Enemy/Snake/Snake_StandardSurface_dead.Snake_StandardSurface_dead" "None"))
      (bind _returnvalue_2 (/ (- (`self.DeadDirectingSec`) _nowsec) (`self.DeadDirectingSec`)))
      (`MaterialInstanceDynamic.SetScalarParameterValue` _returnvalue "Opacity" _returnvalue_2)
      (`FXSystemComponent.SetFloatParameter` (`self.PT_EnemyAura`) "SpawnRate" _returnvalue_2))))

(fn `SnakeRush`
  (if (`self.AttackStartedFlag`)
    (if (`self.FinActionFlag`)
      (`self.Rush Base` true)
      (bind _fin (`self.SecCnt` (`self.RushAfterSec`)))
      (if _fin
        (`self.FinAction`))
      (else
        (`self.Rush Base` false)
        (bind _fin_2 (`self.SecCnt` (`self.RushSec`)))
        (if _fin_2
          (set `self.FinActionFlag` true)
          (set `self.ATK` 0.0))))
    (else
      ;[1 1 1] 方向決定
      (`self.Rotate To Face Player XY plane`)
      (bind _fin_3 (`self.SecCnt` (`self.RushPrepareSec`)))
      (if _fin_3
        (set `self.ATK` (`self.RushAttackNum`))
        (set `self.RushVector` (`self.GetActorForwardVector`))
        (set `self.AttackStartedFlag` true)))))

(fn `UserConstructionScript`
  (`parent.UserConstructionScript`))