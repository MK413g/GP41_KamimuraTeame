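; Base enemy Blueprint that handles attacking the player, taking hits and knockback.
; Attack subtracts ATK from the player's Hp, while HitPlayerAttack lowers enemy HP, stores the hit vector and passes hit and dead flags to the BP_EnemyBaseAI controller.
; KnockBack offsets the actor along that vector scaled by KnockBackPower, resetting power and clearing the Blackboard hit flag when power runs out.
; Flinch is an empty stub.
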(event `self.ReceiveBeginPlay`)

(fn `Attack`
  (params (Player :type "/Game/Main/BP/Player/BP_Player Object Reference"))
  (set `/Game/Main/BP/Player/BP_Player.hp` (- (`/Game/Main/BP/Player/BP_Player.hp` Player) (`self.ATK`)) Player))

(fn `Flinch`)

(fn `HitPlayerAttack`
  (params (AttackVector :type "Vector Structure") (Damage :type "Float (double-precision)"))
  (set `self.MagatamaHitVector` AttackVector)
  (bind _output_get (set `self.HP` (- (`self.HP`) Damage)))
  (set `self.HitFlag` true)
  (bind _returnvalue (<= _output_get 0.0))
  (set `self.DeadFlag` _returnvalue)
  (bind _asbp_enemy_base_ai (cast `/Game/Main/BP/Enemy/ST_EnemyAIBase/BP_EnemyBaseAI` (`self.GetController`)))
  (`/Game/Main/BP/Enemy/ST_EnemyAIBase/BP_EnemyBaseAI.SetHitFlag` _asbp_enemy_base_ai true)
  (`/Game/Main/BP/Enemy/ST_EnemyAIBase/BP_EnemyBaseAI.SetDeadFlag` _asbp_enemy_base_ai _returnvalue))

(fn `KnockBack`
  (locals (`HitFlag Key Name` :type Name :default "HitFlag"))
  (`self.K2_SetActorLocation` (+ (`self.K2_GetActorLocation`) (* (`self.MagatamaHitVector`) (`self.KnockBackPower`))))
  (if (<= (- (`self.KnockBackPower`) 1.0) 0.0)
    (set `self.KnockBackPower` 60.0)
    (`BlackboardComponent.SetValueAsBool` (`AIBlueprintHelperLibrary.GetBlackboard` (`self.GetController`)) (`local.HitFlag Key Name`) false)))

(fn `UserConstructionScript`)