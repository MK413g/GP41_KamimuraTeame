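; BP_LaserCopy is an enemy laser beam actor that fires forward, damages the player once, then destroys itself.
; While firing, Tick grows the beam's length and runs a multi line trace, stopping it at blocking hits not tagged Enemy.
; The trace drives the Niagara beam's end and width and places the impact effect.
; After ShotSec the beam stops tracing and narrows until the actor is destroyed.
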(event `self.ReceiveBeginPlay`
  (`FXSystemComponent.SetColorParameter` (`self.NiagaraLaserImpact`) "Colour" (`self.BeamColor`))
  (`FXSystemComponent.SetColorParameter` (`self.NS_LaserCopy`) "Colour" (`self.BeamColor`)))

(event `self.ReceiveTick`
  (params (DeltaSeconds :type "Float (single-precision)"))
  (bind _returnvalue (`self.K2_GetActorLocation`))
  (bind _returnvalue_2 (+ _returnvalue (* (`self.GetActorForwardVector`) (`self.Distance`))))
  (if (`self.NowShotFlag`)
    (`|ExecutionSequence`
      (:`then_0`
        (set `self.TraceEnd` _returnvalue_2)
        (bind (_outhits _returnvalue_3) (`KismetSystemLibrary.LineTraceMultiForObjects` _returnvalue _returnvalue_2 (`self.TraceObject Types`)))
        (if _returnvalue_3
          (for _array_element _outhits
            (if (not (`self.OnHit`))
              (if (`GameplayStatics.BreakHitResult` _array_element)
                (set `self.OnHit` (not (`self.ActorHasTag` (`.HitActor` (`GameplayStatics.BreakHitResult` _array_element)) "Enemy")))
                (else
                  (set `self.OnHit` false)))
              (`|ExecutionSequence`
                (:`then_0`
                  (if (`self.OnHit`)
                    (set `self.HitLocation` (`.Location` (`GameplayStatics.BreakHitResult` _array_element))))
                  (`FXSystemComponent.SetVectorParameter` (`self.NS_LaserCopy`) "LaserEnd" (select `bool` (`self.OnHit`) :`false` (`self.TraceEnd`) :`true` (`self.HitLocation`)))
                  (`SceneComponent.SetVisibility` (`self.NiagaraLaserImpact`) (`self.OnHit`) true)
                  (`SceneComponent.K2_SetWorldLocation` (`self.NiagaraLaserImpact`) (`self.HitLocation`) false false)
                  (`FXSystemComponent.SetFloatParameter` (`self.NS_LaserCopy`) "Beam Width" (`self.Width`))
                  (if (`self.OnHit`)
                    (set `self.Distance` (`KismetMathLibrary.VSize` (- (`self.HitLocation`) (`self.K2_GetActorLocation`))))))
                (:`then_1`
                  (if (`self.OnHit`)
                    (if (`self.ActorHasTag` (`.HitActor` (`GameplayStatics.BreakHitResult` _array_element)) "Player")
                      (if (not (`self.FirstHit`))
                        (bind _asbp_player (cast `/Game/Main/BP/Player/BP_Player` (`.HitActor` (`GameplayStatics.BreakHitResult` _array_element))))
                        (`PlayerBase.SetDamage` _asbp_player (`self.Damage`) (0.0 0.0 0.0) 0.0)
                        (set `self.FirstHit` true))))))))))
      (:`then_1`
        (if (< (`self.Distance`) (`self.MaxDistance`))
          (set `self.Distance` (+ (`self.Distance`) (* DeltaSeconds (`self.BeamSpeed`))))))
      (:`then_2`
        (if (< (`self.Width`) (`self.MaxWidth`))
          (bind _output_get (set `self.Width` (+ (`self.Width`) (* (`self.MaxWidth`) (`GameplayStatics.GetWorldDeltaSeconds`)))))
          (if (< _output_get (`self.MaxWidth`))
            (set `self.Width` (`self.MaxWidth`)))))
      (:`then_3`
        (set `self.OnHit` false)
        (bind _output_get_2 (set `self.SecCntNum` (+ (`self.SecCntNum`) (`GameplayStatics.GetWorldDeltaSeconds`))))
        (if (> _output_get_2 (`self.ShotSec`))
          (set `self.NowShotFlag` false))))
    (elif (> (`self.Width`) 0.0)
      (bind _output_get_3 (set `self.Width` (- (`self.Width`) (* (`self.DecrementWidth`) (`GameplayStatics.GetWorldDeltaSeconds`)))))
      (if (> _output_get_3 0.0)
        (`FXSystemComponent.SetFloatParameter` (`self.NS_LaserCopy`) "Beam Width" (`self.Width`))
        (else
          (`self.K2_DestroyActor`))))))

(fn `UserConstructionScript`)