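; Karakasa enemy character that damages the player on capsule contact and supports knockback and a fade-out death.
; Tick reports zero HP to BP_KarakasaAI as a dead flag.
; Knockback offsets the actor along the Magatama hit vector and clears a blackboard hit flag at low power.
; Each death call lowers dynamic-material opacity and aura flames, finally destroying those components and the capsule; RushCharge is an empty stub.
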(event `self.ReceiveTick`
  (params (DeltaSeconds :type "Float (single-precision)"))
  (bind _asbp_karakasa_ai (cast `/Game/Main/BP/Enemy/ST_Karakasa/BP_KarakasaAI` (`AIBlueprintHelperLibrary.GetAIController` self)))
  (`/Game/Main/BP/Enemy/ST_EnemyAIBase/BP_EnemyBaseAI.SetDeadFlag` _asbp_karakasa_ai (<= (`self.HP`) 0.0)))

(event `self.Capsule.OnComponentHit`
  (params (HitComponent :type "PrimitiveComponent Object Reference") (OtherActor :type "Actor Object Reference") (OtherComp :type "PrimitiveComponent Object Reference") (NormalImpulse :type "Vector Structure") (Hit :type "HitResult Structure (by ref)"))
  (bind _atk (`self.ATK`))
  ;[1 1 1] 攻撃等
  (if (`self.ActorHasTag` OtherActor "Player")
    (bind _asbp_player (cast `/Game/Main/BP/Player/BP_Player` OtherActor))
    (if (> _atk 0.0)
      (`PlayerBase.SetDamage` _asbp_player _atk (`KismetMathLibrary.Conv_RotatorToVector` (`self.K2_GetActorRotation` self)) 0.0))
    (elif (`self.ActorHasTag` OtherActor "Magatama")
      _)))

(fn `Karakasa Dead`
  (bind _deadalphanum (`self.DeadAlphaNum`))
  (bind _returnvalue (- _deadalphanum 0.1))
  (if (> (`self.DeadAlphaNum`) 0.0)
    (bind _returnvalue_2 (`PrimitiveComponent.CreateDynamicMaterialInstance` (`self.karakasa_model_10_19`) 0 "/Game/Main/Meshes/Enemy/KarakasaObake/karakasasobake_material1_Delete.karakasasobake_material1_Delete" "None"))
    (`MaterialInstanceDynamic.SetScalarParameterValue` _returnvalue_2 "Opacity" _deadalphanum)
    (`FXSystemComponent.SetFloatParameter` (`self.PT_EnemyAura_3`) "FlamesRate" _returnvalue)
    (`FXSystemComponent.SetFloatParameter` (`self.PT_EnemyAura_2`) "FlamesRate" _returnvalue)
    (bind _output_get (set `self.DeadAlphaNum` (- _deadalphanum 0.01)))
    (if (<= _output_get 0.0)
      (`ActorComponent.K2_DestroyComponent` (`self.karakasa_model_10_19`))
      (`ActorComponent.K2_DestroyComponent` (`self.Capsule`))
      (`ActorComponent.K2_DestroyComponent` (`self.PT_EnemyAura_3`))
      (`ActorComponent.K2_DestroyComponent` (`self.PT_EnemyAura_2`)))))

(fn `Karakasa_KnockBack`
  (locals (HitFlagKeyName :type Name :default "HitFlag"))
  (bind _returnvalue (- (`self.KnockBackPower_`) 1.0))
  (`self.K2_SetActorLocation` (+ (`self.K2_GetActorLocation`) (* (`self.MagatamaHitVector`) (`self.KnockBackPower_`))))
  (if (<= _returnvalue 0.0)
    (set `self.KnockBackPower_` _returnvalue)
    (`BlackboardComponent.SetValueAsBool` (`AIBlueprintHelperLibrary.GetBlackboard` (`self.GetController`)) (`local.HitFlagKeyName`) false)))

(fn `RushCharge`
  (locals (NewLocalVar_0 :type "BlackboardKeySelector Structure")))

(fn `UserConstructionScript`
  (`parent.UserConstructionScript`))