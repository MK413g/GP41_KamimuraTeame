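; BP_Snail is a snail enemy that chases the player, rushes, fires water bullets, flinches and fades out on death.
; BeginPlay loads its stats from DT_SnailStatus and sets up scale and aura.
; Each action is a SecCnt-timed state function; attacks face the player while preparing, then lock direction.
; FinAction resets attack state and asks BP_SnailAI for the next action, starting the charge sound when needed.
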(event `self.ReceiveBeginPlay`
  (bind _pt_enemyaura (`self.PT_EnemyAura`))
  (`|ExecutionSequence`
    (:`then_0`
      (`self.FinAction`)
      (bind _returnvalue (`|GetDataTableRow` "/Game/Main/DataTable/DT_SnailStatus.DT_SnailStatus" "SnailState")
        (:`then`
          (set `self.HP` (break `/Game/Main/BP/Enemy/Snail/ST_SnailStatus` _returnvalue))
          (set `self.MoveSpeed_Sec` (`.MoveSpeed_38_D2B7BE2D4875D1C1D3BB479A2B5DA3E0` (break `/Game/Main/BP/Enemy/Snail/ST_SnailStatus` _returnvalue)))
          (set `self.RotateSpeed_Sec` (`.RotateSpeed_37_3CB5073D49250B92406A308753F0C366` (break `/Game/Main/BP/Enemy/Snail/ST_SnailStatus` _returnvalue)))
          (set `self.RushSpeed` (`.RushSpeed_36_0739916243CFA30A1E13DAA08C76ECE9` (break `/Game/Main/BP/Enemy/Snail/ST_SnailStatus` _returnvalue)))
          (set `self.RushPrepareSec` (`.RushPrepareSec_18_16776D5645EAB20195AB3BB6786874AD` (break `/Game/Main/BP/Enemy/Snail/ST_SnailStatus` _returnvalue)))
          (set `self.RushSec` (`.RushSec_11_AB02E68548097F459979089B3829EDCE` (break `/Game/Main/BP/Enemy/Snail/ST_SnailStatus` _returnvalue)))
          (set `self.RushAfterSec` (`.AfterRushSec_17_7BBDDE1147BF97109E0DA0BB10737B88` (break `/Game/Main/BP/Enemy/Snail/ST_SnailStatus` _returnvalue)))
          (set `self.RushAttackNum` (`.RushAttackNum_19_BC100696497CE9C4D28956A2CAC31D15` (break `/Game/Main/BP/Enemy/Snail/ST_SnailStatus` _returnvalue)))
          (set `self.WatterBulletPreapreSec` (`.WaterBulletPrepareSec_45_B4D154714D4A676881844B932A02697E` (break `/Game/Main/BP/Enemy/Snail/ST_SnailStatus` _returnvalue)))
          (set `self.AfterShotWaterBulletSec` (`.AfterWaterBulletShotSec_47_9132FF5643AC4B5C9B5E35A537AC9DF9` (break `/Game/Main/BP/Enemy/Snail/ST_SnailStatus` _returnvalue)))
          (set `self.WaterBulletScale` (`.WaterBulletScale_67_E3DDC81141EA3D0D2601BE9F2D68E355` (break `/Game/Main/BP/Enemy/Snail/ST_SnailStatus` _returnvalue)))
          (set `self.WaterBulletAttackNum` (`.WaterBulletAttackNum_51_DFAE1E66452F11444087469E4F98AD59` (break `/Game/Main/BP/Enemy/Snail/ST_SnailStatus` _returnvalue)))
          (set `self.WaterBulletSpeed` (`.WaterBulletSpeed_52_5AC1BC134359E19FAF3D19BE0D0C736E` (break `/Game/Main/BP/Enemy/Snail/ST_SnailStatus` _returnvalue)))
          (set `self.WaterBulletLifeTime` (`.WaterBulletLifeSec_54_6812D13142422F0CF871EEB2611C0673` (break `/Game/Main/BP/Enemy/Snail/ST_SnailStatus` _returnvalue)))
          (set `self.FlinchSec` (`.FlinchSec_57_FE17E7DF45C407F8125570B754756CBF` (break `/Game/Main/BP/Enemy/Snail/ST_SnailStatus` _returnvalue)))
          (set `self.BeFlinchDamage` (`.FlinchHitNum_60_9D929A004895E8FF1A423296D74DD7D5` (break `/Game/Main/BP/Enemy/Snail/ST_SnailStatus` _returnvalue)))
          (set `self.CollisionSize` (`.CollisionSize_64_BFE0BD8045B11B46AAFA8CACBC05E915` (break `/Game/Main/BP/Enemy/Snail/ST_SnailStatus` _returnvalue))))))
    (:`then_1`
      (`FXSystemComponent.SetActorParameter` _pt_enemyaura "VertSurfaceActor" self)
      (`SceneComponent.SetRelativeScale3D` _pt_enemyaura (0.25 0.5 0.25))
      (`FXSystemComponent.SetFloatParameter` _pt_enemyaura "SpawnRate" 0.0))
    (:`then_2`
      (`self.SetActorScale3D` (`self.CollisionSize`))
      (`SceneComponent.SetWorldScale3D` (`self.3D_Snail`) (30.0 30.0 30.0))
      (`SceneComponent.SetWorldScale3D` (`self.PT_EnemyAura`) (1.0 1.0 1.0))
      (`parent.ReceiveBeginPlay`))))

(event `self.ReceiveTick`
  (params (DeltaSeconds :type "Float (single-precision)"))
  (`parent.ReceiveTick` DeltaSeconds))

(event `self.ReceiveActorBeginOverlap`
  (params (OtherActor :type "Actor Object Reference")))

(fn `FinAction`
  (bind _bulletchargese (`self.BulletChargeSE`))
  (set `self.ATK` 0.0)
  (set `self.TimeCnt` 0.0)
  (set `self.AttackStartedFlag` false)
  (set `self.FinActionFlag` false)
  (set `self.ShotWaterBulletFlag` false)
  (bind _asbp_snail_ai (cast `/Game/Main/BP/Enemy/Snail/BP_SnailAI` (`AIBlueprintHelperLibrary.GetAIController` self)))
  (`/Game/Main/BP/Enemy/Snail/BP_SnailAI.Set Next Action` _asbp_snail_ai)
  (bind _snail_action (`/Game/Main/BP/Enemy/Snail/BP_SnailAI.SNAIL_ACTION` _asbp_snail_ai))
  (set `self.AttackMotionFlag` (`|EnumInequality` _snail_action "NewEnumerator2"))
  (if (`|EnumEquality` _snail_action "NewEnumerator1")
    (`ActorComponent.Activate` (`self.BulletChargeSE`) true)
    (`AudioComponent.Play` _bulletchargese 0.0)
    (`AudioComponent.SetVolumeMultiplier` _bulletchargese 1.0)))

(fn `MoveToPlayerSnail`
  (if (`self.FinActionFlag`)
    (`self.FinAction`)
    (else
      (`self.MoveToPlayer`))))

(fn `Snail_Rush`
  (if (`self.AttackStartedFlag`)
    (if (`self.FinActionFlag`)
      (set `self.ATK` 0.0)
      (`self.Rush Base` true)
      (bind _fin (`self.SecCnt` (`self.RushAfterSec`)))
      (if _fin
        (`self.FinAction`))
      (else
        (`self.Rush Base` false)
        (bind _fin_2 (`self.SecCnt` (`self.RushSec`)))
        (if _fin_2
          (set `self.FinActionFlag` true)
          (set `self.ATK` 0.0))))
    (else
      (`self.Rotate To Face Player XY plane`)
      (bind _fin_3 (`self.SecCnt` (`self.RushPrepareSec`)))
      (if _fin_3
        (set `self.ATK` (`self.RushAttackNum`))
        (set `self.RushVector` (`self.GetActorForwardVector`))
        (set `self.AttackStartedFlag` true)
        (`SoundManagerBase.PlaySoundLocation` "/Game/Main/Sound/SE/Enemey/SE_Rush.SE_Rush" "SE" (`self.K2_GetActorLocation`) 1.0 1.0 0.0 null null)))))

(fn `Snail_ShotWaterBullet`
  (bind (_returnvalue_location _returnvalue_rotation) (`KismetMathLibrary.BreakTransform` (`self.GetTransform`)))
  (if (`self.ShotWaterBulletFlag`)
    (bind _fin (`self.SecCnt` (`self.AfterShotWaterBulletSec`)))
    (`AudioComponent.Stop` (`self.BulletChargeSE`))
    (if _fin
      (`self.FinAction`))
    (else
      (`self.Rotate To Face Player XY plane`)
      (bind _fin_2 (`self.SecCnt` (`self.WatterBulletPreapreSec`)))
      (if _fin_2
        (bind _returnvalue (`|SpawnActorFromClass` "/Game/Main/BP/Enemy/BP_WaterBullet.BP_WaterBullet_C" (`KismetMathLibrary.ComposeTransforms` (`KismetMathLibrary.Conv_VectorToTransform` (`self.WaterBulletSpawnPos`)) (`KismetMathLibrary.MakeTransform` _returnvalue_location _returnvalue_rotation (`self.WaterBulletScale`))) "Undefined" "OverrideRootScale" null null))
        (set `/Game/Main/BP/Enemy/BP_WaterBullet.ATK` (`self.WaterBulletAttackNum`) _returnvalue)
        (set `/Game/Main/BP/Enemy/BP_WaterBullet.MoveVec` (`self.GetActorForwardVector`) _returnvalue)
        (set `/Game/Main/BP/Enemy/BP_WaterBullet.Speed` (`self.WaterBulletSpeed`) _returnvalue)
        (set `/Game/Main/BP/Enemy/BP_WaterBullet.LifeSec` (`self.WaterBulletLifeTime`) _returnvalue)
        (set `self.ShotWaterBulletFlag` true)))))

(fn `SnailDead`
  (if (not (`self.FinDeadDirectingFlag`))
    (bind (_fin _nowsec) (`self.SecCnt` (`self.DeadDirectingSec`)))
    (if _fin
      (`ActorComponent.K2_DestroyComponent` (`self.3D_Snail`))
      (`ActorComponent.K2_DestroyComponent` (`self.PT_EnemyAura`))
      (set `self.FinDeadDirectingFlag` true)
      (else
        (bind _returnvalue (`PrimitiveComponent.CreateDynamicMaterialInstance` (`self.3D_Snail`) 0 "/Game/Main/Meshes/Enemy/Carp/lambert3_Dead.lambert3_Dead" "None"))
        (bind _returnvalue_2 (/ (- (`self.DeadDirectingSec`) _nowsec) (`self.DeadDirectingSec`)))
        (`MaterialInstanceDynamic.SetScalarParameterValue` _returnvalue "Opacity" _returnvalue_2)
        (`FXSystemComponent.SetFloatParameter` (`self.PT_EnemyAura`) "SpawnRate" _returnvalue_2)))))

(fn `SnailFlinch`
  (`self.Flinch`)
  (if (not (`self.FlinchFlag`))
    (`self.FinAction`)))

(fn `UserConstructionScript`
  (`parent.UserConstructionScript`))