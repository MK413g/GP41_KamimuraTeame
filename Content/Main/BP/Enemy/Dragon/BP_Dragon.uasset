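; Dragon enemy with three timed attacks: a rush, a water breath and an onibi (will-o'-the-wisp) summon, tuned from DT_DragonState.
; Each attack turns toward the player while preparing, then runs on SecCnt timers and asks BP_DragonAI to select the next.
; The rush sets ATK for contact damage, breath toggles a child BP_WaterBreath, and summons spawn onibi at intervals along an arc.
; Tick lifts the dragon whenever it drops below a minimum height.
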(event `self.ReceiveBeginPlay`
  (`self.FinAttack`)
  (bind _returnvalue (`|GetDataTableRow` "/Game/Main/DataTable/DT_DragonState.DT_DragonState" "DragonState")
    (:`then`
      (set `self.HP` (break `/Game/Main/BP/Enemy/Dragon/ST_DragonState` _returnvalue))
      (set `self.MoveSpeed_Sec` (`.MoveSpeed_38_D2B7BE2D4875D1C1D3BB479A2B5DA3E0` (break `/Game/Main/BP/Enemy/Dragon/ST_DragonState` _returnvalue)))
      (set `self.RotateSpeed_Sec` (`.RotateSpeed_37_3CB5073D49250B92406A308753F0C366` (break `/Game/Main/BP/Enemy/Dragon/ST_DragonState` _returnvalue)))
      (set `self.RushSpeed` (`.RushSpeed_36_0739916243CFA30A1E13DAA08C76ECE9` (break `/Game/Main/BP/Enemy/Dragon/ST_DragonState` _returnvalue)))
      (set `self.RushPrepareTime` (`.RushPrepareSec_18_16776D5645EAB20195AB3BB6786874AD` (break `/Game/Main/BP/Enemy/Dragon/ST_DragonState` _returnvalue)))
      (set `self.RushTime` (`.RushSec_11_AB02E68548097F459979089B3829EDCE` (break `/Game/Main/BP/Enemy/Dragon/ST_DragonState` _returnvalue)))
      (set `self.AfterRushTime` (`.AfterRushSec_17_7BBDDE1147BF97109E0DA0BB10737B88` (break `/Game/Main/BP/Enemy/Dragon/ST_DragonState` _returnvalue)))
      (set `self.RushAttackNum` (`.RushAttackNum_19_BC100696497CE9C4D28956A2CAC31D15` (break `/Game/Main/BP/Enemy/Dragon/ST_DragonState` _returnvalue)))
      (set `self.WaterBreathPrepareSec` (`.WaterBreathPrepareSec_23_B4D154714D4A676881844B932A02697E` (break `/Game/Main/BP/Enemy/Dragon/ST_DragonState` _returnvalue)))
      (set `self.BreathShotSec` (`.WaterBreathShotSec_29_9132FF5643AC4B5C9B5E35A537AC9DF9` (break `/Game/Main/BP/Enemy/Dragon/ST_DragonState` _returnvalue)))
      (set `self.AfterWaterBreathSec` (`.AfterWaterBreathSec_30_432902DB48D0ABDA1477718E0DE2E103` (break `/Game/Main/BP/Enemy/Dragon/ST_DragonState` _returnvalue)))
      (bind _asbp_water_breath (cast `/Game/Main/BP/Enemy/BP_WaterBreath` (`ChildActorComponent.ChildActor` (`self.BP_WaterBreath`))))
      (set `/Game/Main/BP/Enemy/BP_WaterBreath.Attack Num` (`.WaterBreathAttackNum_21_DFAE1E66452F11444087469E4F98AD59` (break `/Game/Main/BP/Enemy/Dragon/ST_DragonState` _returnvalue)) _asbp_water_breath)
      (set `self.OnibiLifeSec` (`.OhnibiLifeSec_32_CDEB45C7407DA9955C7CCFA302131C57` (break `/Game/Main/BP/Enemy/Dragon/ST_DragonState` _returnvalue)))
      (set `self.OnibiSpeed` (`.OnibiSpeed_33_D3804AB94A92515037214899C2A0E642` (break `/Game/Main/BP/Enemy/Dragon/ST_DragonState` _returnvalue)))
      (set `self.OnibiAttackNum` (`.OnibiAttackNum_31_E60E29714A9D500E177737AFA7E0ECAF` (break `/Game/Main/BP/Enemy/Dragon/ST_DragonState` _returnvalue)))
      (set `self.OnibiSpawnInterval` (`.OnibiSpawnIntervalSec_41_749E430A470287E88A33CAB7FE2E2741` (break `/Game/Main/BP/Enemy/Dragon/ST_DragonState` _returnvalue)))
      (set `self.CanSpawnOnibiNum` (`.OnibiSpawnNum_44_B77D6444499343B6C912CEBADDBB0DEC` (break `/Game/Main/BP/Enemy/Dragon/ST_DragonState` _returnvalue)))
      (`parent.ReceiveBeginPlay`))))

(event `self.ReceiveTick`
  (params (DeltaSeconds :type "Float (single-precision)"))
  (bind (_returnvalue_x _returnvalue_y _returnvalue_z) (`KismetMathLibrary.BreakVector` (`self.K2_GetActorLocation`)))
  (bind (_returnvalue_x_2 _returnvalue_y_2 _returnvalue_z_2) (`KismetMathLibrary.BreakVector` (`self.K2_GetActorLocation`)))
  (if (< _returnvalue_z_2 400.0)
    (`self.K2_SetActorLocation` (`KismetMathLibrary.MakeVector` _returnvalue_x_2 _returnvalue_y_2 (+ _returnvalue_z_2 (* (`GameplayStatics.GetWorldDeltaSeconds`) 1000.0))))
    (if (>= _returnvalue_z 400.0)
      (`self.K2_SetActorLocation` (`KismetMathLibrary.MakeVector` _returnvalue_x _returnvalue_y 400.0))))
  (`parent.ReceiveTick` 0.0))

(event `self.Capsule.OnComponentBeginOverlap`
  (params (OverlappedComponent :type "PrimitiveComponent Object Reference") (OtherActor :type "Actor Object Reference") (OtherComp :type "PrimitiveComponent Object Reference") (OtherBodyIndex :type Integer) (bFromSweep :type Boolean) (SweepResult :type "HitResult Structure (by ref)"))
  (bind _atk (`self.ATK`))
  (if (`self.ActorHasTag` OtherActor "Player")
    (bind _asbp_player (cast `/Game/Main/BP/Player/BP_Player` OtherActor))
    (if (> _atk 0.0)
      (`PlayerBase.SetDamage` _asbp_player _atk (0.0 0.0 0.0) 0.0))))

(event `self.Dragon.OnComponentHit`
  (params (HitComponent :type "PrimitiveComponent Object Reference") (OtherActor :type "Actor Object Reference") (OtherComp :type "PrimitiveComponent Object Reference") (NormalImpulse :type "Vector Structure") (Hit :type "HitResult Structure (by ref)"))
  (bind _atk (`self.ATK`))
  (if (`self.ActorHasTag` OtherActor "Player")
    (bind _asbp_player (cast `/Game/Main/BP/Player/BP_Player` OtherActor))
    (if (> _atk 0.0)
      (`PlayerBase.SetDamage` _asbp_player _atk (0.0 0.0 0.0) 0.0))))

(fn `AfterDragonRush`)

(fn `AftwerWaterBreath`)

(fn `Dragon Rush`
  (bind (_returnvalue_x _returnvalue_y _returnvalue_z) (`KismetMathLibrary.BreakVector` (`self.K2_GetActorLocation`)))
  (if (`self.FinAttackFlag`)
    (bind _fin (`self.SecCnt` (`self.AfterRushTime`)))
    (if _fin
      (`self.FinAttack`))
    (else
      (`self.K2_SetActorLocation` (+ (`self.K2_GetActorLocation`) (* (`self.RushVector`) (* (* (`GameplayStatics.GetWorldDeltaSeconds`) 2.0) (`self.RushSpeed`)))))
      (bind _fin_2 (`self.SecCnt` (`self.RushTime`)))
      (if (or _fin_2 (< _returnvalue_z 270.0))
        (set `self.ATK` 0.0)
        (set `self.FinAttackFlag` true)))))

(fn `DragonRushPrepare`
  (`self.Rotate To Face Player XY plane`)
  (bind _fin (`self.SecCnt` (`self.RushPrepareTime`)))
  (if _fin
    (set `self.AttackStartedFlag` true)
    (set `self.RushVector` (`self.GetActorForwardVector`))
    (set `self.ATK` (`self.RushAttackNum`))))

(fn `FinAttack`
  (bind _asbp_dragon_ai (cast `/Game/Main/BP/Enemy/Dragon/BP_DragonAI` (`AIBlueprintHelperLibrary.GetAIController` self)))
  (`/Game/Main/BP/Enemy/Dragon/BP_DragonAI.Set SelectAttackNum` _asbp_dragon_ai)
  (set `self.AttackStartedFlag` false)
  (set `self.FinAttackFlag` false))

(fn `Stay`)

(fn `SummonOnibi`
  (locals (SpawnOnibiPos :type "Vector Structure") (SpawnOnibiPosToDragonDistanse :type "Float (double-precision)" :default 1000.0))
  (if (`self.CanOnibiSpawnFlag`)
    (bind _output_get (set `local.SpawnOnibiPos` (+ (`self.K2_GetActorLocation`) (* (`KismetMathLibrary.RotateAngleAxis` (`self.GetActorRightVector`) (* (/ 180.0 (`KismetMathLibrary.Conv_IntToDouble` (- (`self.CanSpawnOnibiNum`) 1))) (`KismetMathLibrary.Conv_IntToDouble` (`self.CanSpawnOnibiNum_Cnt`))) (`self.GetActorForwardVector`)) (`local.SpawnOnibiPosToDragonDistanse`)))))
    (bind _returnvalue (`|SpawnActorFromClass` "/Game/Main/BP/Enemy/BP_Onibi.BP_Onibi_C" (`KismetMathLibrary.Conv_VectorToTransform` _output_get) "Undefined" "OverrideRootScale" null null))
    (set `/Game/Main/BP/Enemy/BP_Onibi.Attack_Num` (`self.OnibiAttackNum`) _returnvalue)
    (set `/Game/Main/BP/Enemy/BP_Onibi.LifeTime` (`self.OnibiLifeSec`) _returnvalue)
    (set `/Game/Main/BP/Enemy/BP_Onibi.Speed` (`self.OnibiSpeed`) _returnvalue)
    (set `self.CanOnibiSpawnFlag` false)
    (bind _output_get_2 (set `self.CanSpawnOnibiNum_Cnt` (+ (`self.CanSpawnOnibiNum_Cnt`) 1)))
    (if (>= _output_get_2 (`self.CanSpawnOnibiNum`))
      (bind _asbp_dragon_ai (cast `/Game/Main/BP/Enemy/Dragon/BP_DragonAI` (`AIBlueprintHelperLibrary.GetAIController` self)))
      (`/Game/Main/BP/Enemy/Dragon/BP_DragonAI.Set SelectAttackNum` _asbp_dragon_ai)
      (set `self.AttackStartedFlag` false)
      (set `self.CanSpawnOnibiNum_Cnt` 0))
    (else
      (bind _fin (`self.SecCnt` (`self.OnibiSpawnInterval`)))
      (if _fin
        (set `self.CanOnibiSpawnFlag` true)))))

(fn `SummonOnibiPrepare`
  (`self.Rotate To Face Player XY plane`)
  (bind _fin (`self.SecCnt` (`self.RushPrepareTime`)))
  (if _fin
    (set `self.AttackStartedFlag` true)
    (set `self.RushVector` (`self.GetActorForwardVector`))))

(fn `UserConstructionScript`
  (`parent.UserConstructionScript`))

(fn `Water Breath Prepare`
  (`self.Rotate to Face Player`)
  (bind _fin (`self.SecCnt` (`self.WaterBreathPrepareSec`)))
  (if _fin
    (set `self.AttackStartedFlag` true)
    (bind _asbp_water_breath (cast `/Game/Main/BP/Enemy/BP_WaterBreath` (`ChildActorComponent.ChildActor` (`self.BP_WaterBreath`))))
    (`/Game/Main/BP/Enemy/BP_WaterBreath.StartBreath` _asbp_water_breath)))

(fn `WaterBreath`
  (locals (NewLocalVar_0 :type "Transform Structure") (SummonOnibiNum :type Integer :default 5))
  (if (`self.FinAttackFlag`)
    (bind _fin (`self.SecCnt` (`self.AfterWaterBreathSec`)))
    (if _fin
      (`self.FinAttack`))
    (else
      (bind _fin_2 (`self.SecCnt` (`self.BreathShotSec`)))
      (if _fin_2
        (bind _asbp_water_breath (cast `/Game/Main/BP/Enemy/BP_WaterBreath` (`ChildActorComponent.ChildActor` (`self.BP_WaterBreath`))))
        (`/Game/Main/BP/Enemy/BP_WaterBreath.StopBreath` _asbp_water_breath)
        (set `self.FinAttackFlag` true)))))