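; BP_Raven is a flying enemy that approaches the player, summons onibi and performs rush attacks.
; BeginPlay loads stats from DT_RavenStatus and precomputes accelerations for the rush's rise-and-dive arc.
; Actions are timed state functions using SecCnt and flags; FinAction resets them and asks BP_RavenAI for the next action.
; Onibi spawn attached in a half circle, rush damage activates after the dive, and death fades model and aura.
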(event `self.ReceiveBeginPlay`
  (bind _pt_enemyaura (`self.PT_EnemyAura`))
  (bind _returnvalue (/ (`self.RushPrepareFlightSec`) 2.0))
  (bind _returnvalue_2 (/ (- (`self.RushPrepareHight`) (`self.RushHight`)) (/ (`self.RushPrepareFlightSec`) 4.0)))
  (bind _returnvalue_3 (/ (* (- (`self.RushPrepareHight`) (`self.BaseStayHight`)) 2.0) _returnvalue_2))
  (`self.FinAction`)
  (`|ExecutionSequence`
    (:`then_0`
      (bind _returnvalue_4 (`|GetDataTableRow` "/Game/Main/DataTable/DT_RavenStatus.DT_RavenStatus" "RavenStatus")
        (:`then`
          (set `self.BaseStayHight` (break `/Game/Main/BP/Enemy/Raven/ST_RavenStatus` _returnvalue_4))
          (set `self.SpawnOnibiNum` (`.SpawnOnibiNum_14_C3EF36F04EC6BCA006AF7F92063999C6` (break `/Game/Main/BP/Enemy/Raven/ST_RavenStatus` _returnvalue_4)))
          (set `self.SpawnOnibiPosToRaveDistance` (`.SpawnOnibiPosToRaveDistance_18_A55F828846CC5E56A79809810C6053D2` (break `/Game/Main/BP/Enemy/Raven/ST_RavenStatus` _returnvalue_4)))
          (set `self.OnibiAttackNum` (`.OnibiAttackNum_20_1ABFBE2A4967EEA7108FF9ACDB5A6C12` (break `/Game/Main/BP/Enemy/Raven/ST_RavenStatus` _returnvalue_4)))
          (set `self.OnibiScale` (`.OnibiScale_67_625C91244F7C6D342C2F76BCE83F6303` (break `/Game/Main/BP/Enemy/Raven/ST_RavenStatus` _returnvalue_4)))
          (set `self.OnibiSpeed` (`.OnibiSpeed_22_A932BD7A4E4BA9426C1350A44D2370C6` (break `/Game/Main/BP/Enemy/Raven/ST_RavenStatus` _returnvalue_4)))
          (set `self.OnibiLifeTime` (`.OnibiLifeTime_24_09A0C69B477BBF994C75C9998D7E63B2` (break `/Game/Main/BP/Enemy/Raven/ST_RavenStatus` _returnvalue_4)))
          (set `self.SummonOnibiPrepareSec` (`.SummonOnibiPrepareSec_26_D441636D4FF6490188BC37AB55E5A43B` (break `/Game/Main/BP/Enemy/Raven/ST_RavenStatus` _returnvalue_4)))
          (set `self.SummonOnibiAfterSec` (`.SummonOnibiAfterSec_28_B9B9EB62493DABDEDCB04F88A9F72A61` (break `/Game/Main/BP/Enemy/Raven/ST_RavenStatus` _returnvalue_4)))
          (set `self.RushPrepareSec` (`.RushPrepareSec_33_E3977E4A45DEFBA7BBF026831D50A88B` (break `/Game/Main/BP/Enemy/Raven/ST_RavenStatus` _returnvalue_4)))
          (set `self.RushSec` (`.RushSec_40_4EC5EF3149990CC1425412AFCA9BC2A3` (break `/Game/Main/BP/Enemy/Raven/ST_RavenStatus` _returnvalue_4)))
          (set `self.RushAfterSec` (`.RushAfterSec_34_A65F42E34F9E65387166B19D7D407683` (break `/Game/Main/BP/Enemy/Raven/ST_RavenStatus` _returnvalue_4)))
          (set `self.RushPrepareHight` (`.RushPrepareHight_35_1D161EED47C46D501D50BF977E330FD8` (break `/Game/Main/BP/Enemy/Raven/ST_RavenStatus` _returnvalue_4)))
          (set `self.RushHight` (`.RushHight_36_F9ECEA2A47D7E2E49A61DD8F691EF4A2` (break `/Game/Main/BP/Enemy/Raven/ST_RavenStatus` _returnvalue_4)))
          (set `self.RushPrepareFlightSec` (`.RushPrepareFlightSec_38_C8699E7042A934071022A8A089FC3866` (break `/Game/Main/BP/Enemy/Raven/ST_RavenStatus` _returnvalue_4)))
          (set `self.RushAttackNum` (`.RushAttackNum_43_D30C90FF44E28A6A4DF3D6BF6A3E8AFB` (break `/Game/Main/BP/Enemy/Raven/ST_RavenStatus` _returnvalue_4)))
          (set `self.RushSpeed` (`.RushSpeed_46_0335E22443C944BD2A187DB81D0243A3` (break `/Game/Main/BP/Enemy/Raven/ST_RavenStatus` _returnvalue_4)))
          (set `self.FlinchSec` (`.FlinchSec_49_CC69A4CB42A4D73820187EA947FD24DD` (break `/Game/Main/BP/Enemy/Raven/ST_RavenStatus` _returnvalue_4)))
          (set `self.BeFlinchDamage` (`.FlinchHitNum_52_934DCD454AC0527FAF3B9EB7C5AA6CB0` (break `/Game/Main/BP/Enemy/Raven/ST_RavenStatus` _returnvalue_4)))
          (set `self.HP` (`.HP_59_4816E2A84D5DC3D6B22F9694BDCA1992` (break `/Game/Main/BP/Enemy/Raven/ST_RavenStatus` _returnvalue_4)))
          (set `self.MoveSpeed_Sec` (`.MoveSpeed_60_2CE512F94BAB13BCECBB6E8C2AD67FB8` (break `/Game/Main/BP/Enemy/Raven/ST_RavenStatus` _returnvalue_4)))
          (set `self.RotateSpeed_Sec` (`.RotateSpeed_61_B7490F10499FCF42F341A78EB96DE618` (break `/Game/Main/BP/Enemy/Raven/ST_RavenStatus` _returnvalue_4)))
          (set `self.CollisionSize` (`.CollisionSize_64_C0C7E3E749890D43D555F19FDA879ADD` (break `/Game/Main/BP/Enemy/Raven/ST_RavenStatus` _returnvalue_4))))))
    (:`then_1`
      (`FXSystemComponent.SetActorParameter` _pt_enemyaura "VertSurfaceActor" self)
      (`SceneComponent.SetRelativeScale3D` _pt_enemyaura (0.2 0.1 0.5))
      (`FXSystemComponent.SetFloatParameter` _pt_enemyaura "SpawnRate" 0.0))
    (:`then_2`
      (`self.SetActorScale3D` (`self.CollisionSize`))
      (`SceneComponent.SetWorldScale3D` (`self.PT_EnemyAura`) (1.0 1.0 1.0))
      (`SceneComponent.SetWorldScale3D` (`self.Raven_model`) (100.0 100.0 100.0)))
    (:`then_3`
      (bind _output_get (set `self.RushPrepareZInitSpeed` (/ (- (`self.RushPrepareHight`) (`self.BaseStayHight`)) (/ (`self.RushPrepareFlightSec`) 4.0))))
      (set `self.RushPrepareNowZSpeed` _output_get)
      (set `self.RushPrepareUpDeceleration` (/ _output_get _returnvalue))
      (set `self.RushPrepareDownAceleration` (/ _returnvalue_2 _returnvalue_3))
      (set `self.RushPrepareDownDeceleration` (/ _returnvalue_2 (- _returnvalue _returnvalue_3)))
      (`parent.ReceiveBeginPlay`))))

(event `self.ReceiveActorBeginOverlap`
  (params (OtherActor :type "Actor Object Reference")))

(event `self.ReceiveTick`
  (params (DeltaSeconds :type "Float (single-precision)"))
  (`parent.ReceiveTick` DeltaSeconds))

(fn `FinAction`
  (set `self.TimeCnt` 0.0)
  (set `self.RushPrepareNowZSpeed` (`self.RushPrepareZInitSpeed`))
  (set `self.AttackStartedFlag` false)
  (set `self.FinActionFlag` false)
  (set `self.FinSpawn` false)
  (set `self.RushPrepareUpCompFlag` false)
  (set `self.RushPrepareUpDownCompFlag` false)
  (bind _asbp_raven_ai (cast `/Game/Main/BP/Enemy/Raven/BP_RavenAI` (`AIBlueprintHelperLibrary.GetAIController` self)))
  (`/Game/Main/BP/Enemy/Raven/BP_RavenAI.Select Next Action` _asbp_raven_ai)
  (set `self.AttackMotionFlag` (not (`|EnumEquality` (`/Game/Main/BP/Enemy/Raven/BP_RavenAI.SELECTED_ACTION` _asbp_raven_ai) "NewEnumerator2"))))

(fn `MoveToPlayerRaven`
  (if (`self.FinActionFlag`)
    (`self.FinAction`)
    (else
      (`self.MoveToPlayer`))))

(fn `RavenDead`
  (if (not (`self.FinDeadDirectingFlag`))
    (bind (_fin _nowsec) (`self.SecCnt` (`self.DeadDirectingSec`)))
    (if _fin
      (`ActorComponent.K2_DestroyComponent` (`self.Raven_model`))
      (`ActorComponent.K2_DestroyComponent` (`self.PT_EnemyAura`))
      (set `self.FinDeadDirectingFlag` true)
      (else
        (bind _returnvalue (`PrimitiveComponent.CreateDynamicMaterialInstance` (`self.Raven_model`) 0 "/Game/Main/Meshes/Enemy/Carp/lambert3_Dead.lambert3_Dead" "None"))
        (bind _returnvalue_2 (/ (- (`self.DeadDirectingSec`) _nowsec) (`self.DeadDirectingSec`)))
        (`MaterialInstanceDynamic.SetScalarParameterValue` _returnvalue "Opacity" _returnvalue_2)
        (`FXSystemComponent.SetFloatParameter` (`self.PT_EnemyAura`) "SpawnRate" _returnvalue_2)))))

(fn `RavenFlinch`
  (`self.Flinch`)
  (if (not (`self.FlinchFlag`))
    (`self.FinAction`)))

(fn `RavenRush`
  (bind (_returnvalue_x _returnvalue_y _returnvalue_z) (`KismetMathLibrary.BreakVector` (`self.K2_GetActorLocation`)))
  (if (`self.FinActionFlag`)
    (`self.RushAfter`)
    (elif (`self.AttackStartedFlag`)
      (if (`self.RushPrepareUpDownCompFlag`)
        (`self.Rush Base` false)
        (bind _fin (`self.SecCnt` (`self.RushSec`)))
        (if _fin
          (set `self.FinActionFlag` true)
          (set `self.ATK` 0.0)
          (if (`self.FinActionFlag`) :!label _label
            (set `self.RushInterruptionZPos` _returnvalue_z)))
        (else
          (`self.RushPrepara_Flight`)
          (goto _label)))
      (else
        (`self.Rotate To Face Player XY plane`)
        (bind _fin_2 (`self.SecCnt` (`self.RushPrepareSec`)))
        (if _fin_2
          (set `self.AttackStartedFlag` true)
          (set `self.RushVector` (`self.GetActorForwardVector`))
          (goto _label))))))

(fn `RushAfter`
  (bind (_returnvalue_x _returnvalue_y _returnvalue_z) (`KismetMathLibrary.BreakVector` (+ (`self.K2_GetActorLocation`) (* (`self.GetActorUpVector`) (* (`self.RushAfterUpInitialSpeed`) (`GameplayStatics.GetWorldDeltaSeconds`) -2.0)))))
  (bind (_returnvalue_x_2 _returnvalue_y_2 _returnvalue_z_2) (`KismetMathLibrary.BreakVector` (+ (`self.K2_GetActorLocation`) (* (`self.GetActorUpVector`) (* (`self.RushAfterUpInitialSpeed`) (`GameplayStatics.GetWorldDeltaSeconds`) 2.0)))))
  (if (> (`self.NowSpeed`) 0.0)
    (`self.Rush Base` true))
  (if (< (`self.BaseStayHight`) (`self.RushInterruptionZPos`))
    (if (> _returnvalue_z (`self.BaseStayHight`))
      (`self.K2_SetActorLocation` (`KismetMathLibrary.MakeVector` _returnvalue_x _returnvalue_y _returnvalue_z)))
    (elif (< _returnvalue_z_2 (`self.BaseStayHight`))
      (`self.K2_SetActorLocation` (`KismetMathLibrary.MakeVector` _returnvalue_x_2 _returnvalue_y_2 _returnvalue_z_2))))
  (bind _fin (`self.SecCnt` (`self.RushAfterSec`)))
  (if _fin
    (`self.FinAction`)))

(fn `RushPrepara_Flight`
  (bind (_returnvalue_x _returnvalue_y _returnvalue_z) (`KismetMathLibrary.BreakVector` (`self.K2_GetActorLocation`)))
  (bind (_returnvalue_x_2 _returnvalue_y_2 _returnvalue_z_2) (`KismetMathLibrary.BreakVector` (`self.K2_GetActorLocation`)))
  (`|ExecutionSequence`
    (:`then_0`
      (`self.Rush Base` false)
      (`self.K2_SetActorLocation` (+ (`self.K2_GetActorLocation`) (* (`self.GetActorUpVector`) (* (`self.RushPrepareNowZSpeed`) (`GameplayStatics.GetWorldDeltaSeconds`) 2.0))))
      (if (>= _returnvalue_z_2 (`self.RushPrepareHight`))
        (set `self.RushPrepareUpCompFlag` true))
      (if (`self.RushPrepareUpCompFlag`)
        (if (>= _returnvalue_z (`self.BaseStayHight`))
          (set `self.RushPrepareNowZSpeed` (- (`self.RushPrepareNowZSpeed`) (* (`self.RushPrepareDownAceleration`) (`GameplayStatics.GetWorldDeltaSeconds`) 2.0)))
          (else
            (set `self.RushPrepareNowZSpeed` (+ (`self.RushPrepareNowZSpeed`) (* (`self.RushPrepareDownDeceleration`) (`GameplayStatics.GetWorldDeltaSeconds`) 2.0)))))
        (else
          (set `self.RushPrepareNowZSpeed` (- (`self.RushPrepareNowZSpeed`) (* (`self.RushPrepareUpDeceleration`) (`GameplayStatics.GetWorldDeltaSeconds`) 2.0))))))
    (:`then_1`
      (bind (_fin _nowsec) (`self.SecCnt` (`self.RushPrepareFlightSec`)))
      (if (>= _nowsec (/ (`self.RushPrepareFlightSec`) 2.0))
        (set `self.RushPrepareUpCompFlag` true))
      (if _fin
        (set `self.RushPrepareUpDownCompFlag` true)
        (set `self.RushPrepareNowZSpeed` (`self.RushPrepareZInitSpeed`))
        (set `self.ATK` (`self.RushAttackNum`))
        (`SoundManagerBase.PlaySoundLocation` "/Game/Main/Sound/SE/Enemey/SE_Rush.SE_Rush" "SE" (`self.K2_GetActorLocation`) 1.0 1.0 0.0 null null)))))

(fn `SummonOnibi`
  (if (`self.AttackStartedFlag`)
    (bind _fin (`self.SecCnt` (`self.SummonOnibiAfterSec`)))
    (if _fin
      (`self.FinAction`))
    (else
      (`|ExecutionSequence`
        (:`then_0`
          (`self.Rotate To Face Player XY plane`)
          (bind _fin_2 (`self.SecCnt` (`self.SummonOnibiPrepareSec`)))
          (if _fin_2
            (set `self.AttackStartedFlag` true)
            (set `self.FinActionFlag` true)))
        (:`then_1`
          ;[1 1 1] 鬼火生成
          (if (not (`self.FinSpawn`))
            (for _index (range (`self.SpawnOnibiNum`))
              (bind _returnvalue (`|SpawnActorFromClass` "/Game/Main/BP/Enemy/BP_Onibi.BP_Onibi_C" (`KismetMathLibrary.MakeTransform` (+ (`self.K2_GetActorLocation`) (* (`KismetMathLibrary.RotateAngleAxis` (`self.GetActorRightVector`) (* (`KismetMathLibrary.Conv_IntToDouble` _index) (/ 180.0 (`KismetMathLibrary.Conv_IntToDouble` (- (`self.SpawnOnibiNum`) 1)))) (`self.GetActorForwardVector`)) (`self.SpawnOnibiPosToRaveDistance`))) (struct) (`self.OnibiScale`)) "Undefined" "OverrideRootScale" null null))
              (set `/Game/Main/BP/Enemy/BP_Onibi.Attack_Num` (`self.OnibiAttackNum`) _returnvalue)
              (set `/Game/Main/BP/Enemy/BP_Onibi.LifeTime` (`self.OnibiLifeTime`) _returnvalue)
              (set `/Game/Main/BP/Enemy/BP_Onibi.MoveStartTime` (`self.SummonOnibiPrepareSec`) _returnvalue)
              (set `/Game/Main/BP/Enemy/BP_Onibi.Speed` (`self.OnibiSpeed`) _returnvalue)
              (`self.K2_AttachToActor` _returnvalue self "None" "KeepWorld" "KeepWorld" "KeepWorld" true))
            (set `self.FinSpawn` true)))))))

(fn `UserConstructionScript`
  (`parent.UserConstructionScript`))