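; BP_Drop_Onibi is a falling onibi enemy hazard that damages the player on touch.
; Tick waits out a start delay, optionally detaches from its parent, then moves straight down until its lifetime expires.
; Sphere overlaps ignore enemy-tagged actors; others stop it, with damage only for a player hit while active.
; Once stopped, it cuts the particle flames, fades the sphere through a dynamic material, then destroys itself.
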(event `self.ReceiveBeginPlay`
  (`FXSystemComponent.SetFloatParameter` (`self.PT_Onibi`) "FlamesRate" 1.0))

(event `self.ReceiveTick`
  (params (DeltaSeconds :type "Float (single-precision)"))
  (if (`self.CanMoveFlag`)
    (if (`self.StopFlag`)
      ;[1 1 1] 消滅演出
      (`FXSystemComponent.SetFloatParameter` (`self.PT_Onibi`) "FlamesRate" 0.0)
      (bind _returnvalue (`PrimitiveComponent.CreateDynamicMaterialInstance` (`self.Sphere1`) 0 "/Game/Main/Material/enemy/OnibiMat.OnibiMat" "None"))
      (`MaterialInstanceDynamic.SetScalarParameterValue` _returnvalue "Opacity" (* (/ (- (`self.Delete time`) (`self.TimeCnt`)) (`self.Delete time`)) 0.5))
      (bind _output_get (set `self.TimeCnt` (+ (`self.TimeCnt`) (`GameplayStatics.GetWorldDeltaSeconds`))))
      (if (>= _output_get (`self.Delete time`))
        (set `self.TimeCnt` 0.0)
        (`self.K2_DestroyActor`))
      (else
        ;[1 1 1] 追尾処理
        (`self.K2_SetActorLocation` (+ (* (0.0 0.0 -1.0) (* (`self.Speed`) (* (`GameplayStatics.GetWorldDeltaSeconds`) 2.0))) (`self.K2_GetActorLocation`)))
        (bind _output_get_2 (set `self.TimeCnt` (+ (`self.TimeCnt`) (`GameplayStatics.GetWorldDeltaSeconds`))))
        (if (>= _output_get_2 (`self.LifeTime`))
          (set `self.StopFlag` true)
          (set `self.TimeCnt` 0.0))))
    (else
      ;[1 1 1] 待機処理
      (bind _output_get_3 (set `self.TimeCnt` (+ (`self.TimeCnt`) (`GameplayStatics.GetWorldDeltaSeconds`))))
      (if (>= _output_get_3 (`self.MoveStartTime`))
        (set `self.CanMoveFlag` true)
        (set `self.TimeCnt` 0.0)
        (if (`self.DetachFlag`)
          (`self.K2_DetachFromActor` "KeepWorld" "KeepWorld" "KeepWorld"))))))

(event `self.Sphere.OnComponentBeginOverlap`
  (params (OverlappedComponent :type "PrimitiveComponent Object Reference") (OtherActor :type "Actor Object Reference") (OtherComp :type "PrimitiveComponent Object Reference") (OtherBodyIndex :type Integer) (bFromSweep :type Boolean) (SweepResult :type "HitResult Structure (by ref)"))
  ;[1 1 1] 衝突処理
  (if (not (or (`self.ActorHasTag` OtherActor "Enemyr") (`self.ActorHasTag` OtherActor "EnemyAttack")))
    (if (and (`self.ActorHasTag` OtherActor "Player") (not (`self.StopFlag`)))
      (bind _asplayer_base (cast `PlayerBase` OtherActor))
      (`PlayerBase.SetDamage` _asplayer_base (`self.Attack_Num`) (0.0 0.0 0.0) 0.0))
    (set `self.TimeCnt` 0.0)
    (set `self.StopFlag` true)))

(fn `UserConstructionScript`)