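; Karakasa umbrella-yokai enemy that charges at the player, loading its stats from DT_KarakasaState before parent BeginPlay.
; Attack functions chain via state flags: face player and pitch down, rush along the flattened up vector until timeout or blocked sweep, then right itself.
; Magatama knockback pushes it with decaying power and rotates it, then resets the attack.
; Death fades the model material and aura particles before destroying those components; Tick only calls the parent.
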(event `self.ReceiveBeginPlay`
  (bind _returnvalue (`|GetDataTableRow` "/Game/Main/DataTable/DT_KarakasaState.DT_KarakasaState" "karakasa_State")
    (:`then`
      (set `self.HP` (break `/Game/Main/BP/Enemy/Karakasa/ST_KarakasaState` _returnvalue))
      (set `self.MoveSpeed_Sec` (`.MoveSpeed_24_330008BB42FF62BFB8D69DA8ED555811` (break `/Game/Main/BP/Enemy/Karakasa/ST_KarakasaState` _returnvalue)))
      (set `self.RotateSpeed_Sec` (`.RotateSpeed_22_7E0ADBDC4694892BA759B49852ADD2F8` (break `/Game/Main/BP/Enemy/Karakasa/ST_KarakasaState` _returnvalue)))
      (set `self.RushSpeed` (`.RushSpeed_23_21D9749B41928E6FB0CF888938235157` (break `/Game/Main/BP/Enemy/Karakasa/ST_KarakasaState` _returnvalue)))
      (set `self.RushPrepareSec` (`.RushPrepareSec_18_B7153FA74BE73529D4D1828B76D48F37` (break `/Game/Main/BP/Enemy/Karakasa/ST_KarakasaState` _returnvalue)))
      (set `self.RushSec` (`.RushSec_14_DAE9CE6C493809B16C3066BF0F1ABB82` (break `/Game/Main/BP/Enemy/Karakasa/ST_KarakasaState` _returnvalue)))
      (set `self.AfterRushTime` (`.AfterRushSec_16_3CB96EF44E95EBB56ED5FF9737D09DC8` (break `/Game/Main/BP/Enemy/Karakasa/ST_KarakasaState` _returnvalue)))
      (set `self.RushAttackNum` (`.RushAttackNum_20_5A97E742467C76D2C47C2FAB2F75A026` (break `/Game/Main/BP/Enemy/Karakasa/ST_KarakasaState` _returnvalue)))
      (`parent.ReceiveBeginPlay`))))

(event `self.ReceiveTick`
  (params (DeltaSeconds :type "Float (single-precision)"))
  (`parent.ReceiveTick` 0.0))

(fn `Karakasa After Rush`
  (bind (_returnvalue_roll _returnvalue_pitch _returnvalue_yaw) (`KismetMathLibrary.BreakRotator` (`self.K2_GetActorRotation`)))
  (if (>= _returnvalue_pitch 0.0)
    (`self.K2_SetActorRotation` (`KismetMathLibrary.MakeRotator` _returnvalue_roll 0.0 _returnvalue_yaw))
    (bind _fin (`self.SecCnt` (`self.AfterRushTime`)))
    (if _fin
      (set `self.FinActionFlag` false)
      (set `self.PrepareFlag` true))
    (else
      (`self.K2_SetActorRotation` (`KismetMathLibrary.MakeRotator` _returnvalue_roll (+ _returnvalue_pitch (* (`GameplayStatics.GetWorldDeltaSeconds`) 180.0)) _returnvalue_yaw)))))

(fn `Karakasa Dead`
  (bind _deadalphanum (`self.DeadAlphaNum`))
  (bind _returnvalue (- _deadalphanum 0.1))
  (if (> (`self.DeadAlphaNum`) 0.0)
    (bind _returnvalue_2 (`PrimitiveComponent.CreateDynamicMaterialInstance` (`self.karakasa_model_10_19`) 0 "/Game/Main/Meshes/Enemy/KarakasaObake/karakasasobake_material1_Delete.karakasasobake_material1_Delete" "None"))
    (`MaterialInstanceDynamic.SetScalarParameterValue` _returnvalue_2 "Opacity" _deadalphanum)
    (`FXSystemComponent.SetFloatParameter` (`self.PT_EnemyAura_3`) "FlamesRate" _returnvalue)
    (`FXSystemComponent.SetFloatParameter` (`self.PT_EnemyAura_2`) "FlamesRate" _returnvalue)
    (bind _output_get (set `self.DeadAlphaNum` (- _deadalphanum 0.01)))
    (if (<= _output_get 0.0)
      (`ActorComponent.K2_DestroyComponent` (`self.karakasa_model_10_19`))
      (`ActorComponent.K2_DestroyComponent` (`self.PT_EnemyAura_3`))
      (`ActorComponent.K2_DestroyComponent` (`self.PT_EnemyAura_2`)))))

(fn `Karakasa Knock Back`
  (locals (HitFlagKeyName :type Name :default "HitFlag") (NewLocalVar_1 :type "Vector Structure" :default (0.0 0.0 1.0)))
  (bind _returnvalue (`self.GetActorForwardVector`))
  (bind _returnvalue_2 (`self.GetActorForwardVector`))
  (bind _magatamahitvector (`self.MagatamaHitVector`))
  (bind _returnvalue_3 (`KismetMathLibrary.RotateAngleAxis` _returnvalue (* 45.0 (`GameplayStatics.GetWorldDeltaSeconds`)) (`KismetMathLibrary.Cross_VectorVector` (`self.GetActorUpVector`) _magatamahitvector)))
  (bind _returnvalue_4 (`KismetMathLibrary.Normal` (`KismetMathLibrary.Conv_Vector2DToVector` (`KismetMathLibrary.Conv_VectorToVector2D` (`self.GetActorForwardVector`)))))
  (bind _returnvalue_5 (`KismetMathLibrary.RotateAngleAxis` _returnvalue_2 (* 45.0 (`GameplayStatics.GetWorldDeltaSeconds`)) (`KismetMathLibrary.Cross_VectorVector` (`self.GetActorForwardVector`) _returnvalue_4)))
  (set `self.KnockBackFlag` true)
  (bind _output_get (set `self.KnockBackPower` (- (`self.KnockBackPower`) (* (`GameplayStatics.GetWorldDeltaSeconds`) 180.0))))
  (if (<= _output_get 0.0)
    (if (>= (`KismetMathLibrary.Dot_VectorVector` _returnvalue_5 _returnvalue_2) (`KismetMathLibrary.Dot_VectorVector` _returnvalue_2 _returnvalue_4))
      (`self.K2_SetActorRotation` (`KismetMathLibrary.Conv_VectorToRotator` _returnvalue_5))
      (else
        (`self.K2_SetActorRotation` (`KismetMathLibrary.Conv_VectorToRotator` _returnvalue_4))
        (bind _fin (`self.SecCnt` (`self.KnockBackTime`)))
        (if _fin
          (set `self.KnockBackPower` 0.0)
          (set `self.AttackStartedFlag` false)
          (set `self.PrepareFlag` true)
          (set `self.FinActionFlag` false)
          (set `self.HitFlag` false)
          (set `self.KnockBackFlag` false))))
    (else
      (`self.K2_SetActorLocation` (+ (`self.K2_GetActorLocation`) (* (`self.MagatamaHitVector`) (`self.KnockBackPower`))))
      (if (>= (`KismetMathLibrary.Dot_VectorVector` _returnvalue_3 _returnvalue) (`KismetMathLibrary.Dot_VectorVector` _returnvalue _magatamahitvector))
        (`self.K2_SetActorRotation` (`KismetMathLibrary.Conv_VectorToRotator` _returnvalue_3))
        (else
          (`self.K2_SetActorRotation` (`KismetMathLibrary.Conv_VectorToRotator` (`self.MagatamaHitVector`))))))))

(fn `KarakasaRush`
  (bind (_sweephitresult _returnvalue) (`self.K2_SetActorLocation` (+ (`self.K2_GetActorLocation`) (* (`self.RushVector`) (* (`GameplayStatics.GetWorldDeltaSeconds`) (`self.RushSpeed`)))) true))
  (bind _fin (`self.SecCnt` (`self.RushSec`)))
  (if (or _fin (not _returnvalue))
    (set `self.AttackStartedFlag` false)
    (set `self.FinActionFlag` true)
    (set `self.ATK` 0.0)))

(fn `Rush Charge`
  (locals (NewLocalVar_0 :type "BlackboardKeySelector Structure"))
  (bind (_returnvalue_roll _returnvalue_pitch _returnvalue_yaw) (`KismetMathLibrary.BreakRotator` (`self.K2_GetActorRotation`)))
  (bind _returnvalue (+ _returnvalue_pitch (* (`GameplayStatics.GetWorldDeltaSeconds`) -180.0)))
  (set `self.PrepareFlag` true)
  (`self.Rotate To Face Player XY plane`)
  (if (> _returnvalue -89.0)
    (`self.K2_SetActorRotation` (`KismetMathLibrary.MakeRotator` _returnvalue_roll _returnvalue _returnvalue_yaw)))
  (bind _fin (`self.SecCnt` (`self.RushPrepareSec`)))
  (if _fin
    (set `self.AttackStartedFlag` true)
    (set `self.PrepareFlag` false)
    (set `self.RushVector` (`KismetMathLibrary.Conv_Vector2DToVector` (`KismetMathLibrary.Conv_VectorToVector2D` (`self.GetActorUpVector`))))
    (set `self.ATK` (`self.RushAttackNum`))))

(fn `UserConstructionScript`
  (`parent.UserConstructionScript`))