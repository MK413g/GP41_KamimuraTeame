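; Base AI controller for enemies that exposes setters for the Blackboard state behind their behavior tree.
; Functions write the flinch, dead and hit bools and the player actor object to Blackboard keys.
; Setting flinch true also calls RunBehaviorTree, while the matching call in SetDeadFlag is disconnected.
; EachBehavior is held with a getter and setter, and SetHitFlag takes its key name from NewLocalVar0.
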(fn `GetBehavior`
  (returns (NewParam :type "BehaviorTree Object Reference"))
  (return (`self.eachBehavior`)))

(fn `Set Flinch Flag`
  (params (flinch_flag :type Boolean))
  (`BlackboardComponent.SetValueAsBool` (`self.Blackboard`) (`self.Flinch Key Name`) flinch_flag)
  (if flinch_flag
    (`self.RunBehaviorTree` null)))

(fn `SetBehavior`
  (params (NewParam :type "BehaviorTree Object Reference"))
  (set `self.eachBehavior` NewParam))

(fn `SetDeadFlag`
  (params (set_flag :type Boolean))
  (`BlackboardComponent.SetValueAsBool` (`self.Blackboard`) (`self.Dead Key Name`) set_flag))

(fn `SetHitFlag`
  (params (`Hit or Not` :type Boolean))
  (locals (NewLocalVar_0 :type Name :default "HitFlag"))
  (`BlackboardComponent.SetValueAsBool` (`self.Blackboard`) (`local.NewLocalVar_0`) `Hit or Not`))

(fn `Update PlayerActor Key`
  (params (NewParam :type "Actor Object Reference"))
  (`BlackboardComponent.SetValueAsObject` (`self.Blackboard`) (`self.PlayerActor Key Name`) NewParam))

(fn `UserConstructionScript`)