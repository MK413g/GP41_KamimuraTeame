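; Base enemy actor providing player tracking, movement, rush attack, damage reaction and an HP bar widget.
; Tick classifies player distance as short, middle or long; box collision damages the player while ATK is positive.
; HitPlayerAttack reduces HP, builds toward flinch, updates the bar and passes hit, flinch and death flags to BP_EnemyBaseAI.
; Per-frame helpers handle capped-rate turning, accelerating rushes, decaying knockback and timed actions.
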(event `self.ReceiveBeginPlay`
  (bind _hp (`self.HP`))
  (bind _returnvalue (`|CreateWidget` "/Game/Main/BP/Widget/EnemyHPbar.EnemyHPbar_C"))
  (bind _output_get (set `self.HPBarWidget` _returnvalue))
  (`UserWidget.AddToViewport` _output_get 0)
  (`/Game/Main/BP/Widget/EnemyHPbar.SetEnemyHP` _output_get _hp _hp)
  (set `self.MaxHP` (`self.HP`)))

(event `self.ReceiveTick`
  (params (DeltaSeconds :type "Float (single-precision)"))
  (bind _returnvalue (- (`self.K2_GetActorLocation` (`GameplayStatics.GetPlayerPawn` 0)) (`self.K2_GetActorLocation`)))
  ;[1 1 1] プレイヤーへの距離とvector取得
  (set `self.ToPlayerVector` (`KismetMathLibrary.Normal` _returnvalue))
  (bind _output_get (set `self.Distance to Player` (`KismetMathLibrary.VSize` _returnvalue)))
  (if (<= _output_get (`self.Longest Short Distance`))
    (set `self.TO_PLAYER_DISTANSE_STATE` "NewEnumerator0")
    (elif (<= _output_get (`self.Longest Middle Distance`))
      (set `self.TO_PLAYER_DISTANSE_STATE` "NewEnumerator1")
      (else
        (set `self.TO_PLAYER_DISTANSE_STATE` "NewEnumerator2"))))
  (set `self.FitlyDistanseFlag` (`|EnumEquality` (`self.FITLY_TO_PLAYER_DISTANSE`) (`self.TO_PLAYER_DISTANSE_STATE`))))

(event `self.BoxCollision.OnComponentBeginOverlap`
  (params (OverlappedComponent :type "PrimitiveComponent Object Reference") (OtherActor :type "Actor Object Reference") (OtherComp :type "PrimitiveComponent Object Reference") (OtherBodyIndex :type Integer) (bFromSweep :type Boolean) (SweepResult :type "HitResult Structure (by ref)"))
  (bind _atk (`self.ATK`))
  (`|ExecutionSequence`
    (:`then_0`
      (if (`self.ActorHasTag` OtherActor "Player")
        (bind _asbp_player (cast `/Game/Main/BP/Player/BP_Player` OtherActor))
        (if (> _atk 0.0)
          (`PlayerBase.SetDamage` _asbp_player _atk (`KismetMathLibrary.Normal` (`self.RushVector`)) 500.0))))))

(event `self.BoxCollision.OnComponentHit`
  (params (HitComponent :type "PrimitiveComponent Object Reference") (OtherActor :type "Actor Object Reference") (OtherComp :type "PrimitiveComponent Object Reference") (NormalImpulse :type "Vector Structure") (Hit :type "HitResult Structure (by ref)"))
  (bind _atk (`self.ATK`))
  (`|ExecutionSequence`
    (:`then_0`
      (if (`self.ActorHasTag` OtherActor "Player")
        (bind _asbp_player (cast `/Game/Main/BP/Player/BP_Player` OtherActor))
        (if (> _atk 0.0)
          (`PlayerBase.SetDamage` _asbp_player _atk (`KismetMathLibrary.Normal` (`self.RushVector`)) 500.0))))
    (:`then_1`
      (if (> (`self.ATK`) 0.0)
        (set `self.FinActionFlag` true)
        (set `self.ATK` 0.0)
        (set `self.TimeCnt` 0.0)))))

(fn `Flinch`
  (bind _fin (`self.SecCnt` (`self.FlinchSec`)))
  (if _fin
    (set `self.FlinchFlag` false)
    (bind _asbp_enemy_base_ai (cast `/Game/Main/BP/Enemy/EnemyBase/BP_EnemyBaseAI` (`self.GetController`)))
    (`/Game/Main/BP/Enemy/EnemyBase/BP_EnemyBaseAI.Set Flinch Flag` _asbp_enemy_base_ai true)))

(fn `HitPlayerAttack`
  (params (AttackVector :type "Vector Structure") (Damage :type "Float (double-precision)"))
  (if (> Damage 0.0)
    (set `self.MagatamaHitVector` AttackVector)
    (bind _output_get (set `self.HP` (- (`self.HP`) Damage)))
    (if (or (`self.FinActionFlag`) (not (`self.AttackMotionFlag`)))
      (bind _output_get_2 (set `self.FlinchCnt` (+ (`self.FlinchCnt`) 1.0)))
      (if (and (>= _output_get_2 (`self.BeFlinchDamage`)) (not (`self.FlinchFlag`)))
        (set `self.FlinchFlag` true)
        (set `self.FlinchCnt` 0.0)
        (bind _asbp_enemy_base_ai (cast `/Game/Main/BP/Enemy/EnemyBase/BP_EnemyBaseAI` (`self.GetController`)))
        (`/Game/Main/BP/Enemy/EnemyBase/BP_EnemyBaseAI.Set Flinch Flag` _asbp_enemy_base_ai true)
        (set `self.TimeCnt` 0.0)))
    (set `self.KnockBackPower` 60.0)
    (set `self.HitFlag` true)
    (bind _returnvalue (<= _output_get 0.0))
    (set `self.DeadFlag` _returnvalue)
    (if (not (> _output_get 0.0))
      (`MainGameEndManager.SetClear`))
    (bind _asbp_enemy_base_ai_2 (cast `/Game/Main/BP/Enemy/EnemyBase/BP_EnemyBaseAI` (`self.GetController`)))
    (`/Game/Main/BP/Enemy/EnemyBase/BP_EnemyBaseAI.SetHitFlag` _asbp_enemy_base_ai_2 true)
    (`/Game/Main/BP/Enemy/EnemyBase/BP_EnemyBaseAI.SetDeadFlag` _asbp_enemy_base_ai_2 _returnvalue)
    (`/Game/Main/BP/Widget/EnemyHPbar.SetEnemyHP` (`self.HPBarWidget`) (`self.HP`) (`self.MaxHP`))))

(fn `KnockBack`
  (locals (`HitFlag Key Name` :type Name :default "HitFlag"))
  (bind _returnvalue (- (`self.KnockBackPower`) 1.0))
  (`self.K2_SetActorLocation` (+ (`self.K2_GetActorLocation`) (* (`self.MagatamaHitVector`) (`self.KnockBackPower`))))
  (if (<= _returnvalue 0.0)
    (set `self.KnockBackPower` 60.0)
    (`BlackboardComponent.SetValueAsBool` (`AIBlueprintHelperLibrary.GetBlackboard` (`self.GetController`)) (`local.HitFlag Key Name`) false)
    (else
      (set `self.KnockBackPower` _returnvalue))))

(fn `MoveToDestinationPos`
  (params (DestinationPos :type "Vector Structure") (`XY Plane` :type Boolean))
  (if `XY Plane`
    (`self.RotateToPosXYPlane` DestinationPos)
    (else
      (`self.RotateToDestinationPos` DestinationPos)))
  (`self.K2_SetActorLocation` (+ (`self.K2_GetActorLocation`) (* (`self.GetActorForwardVector`) (* (`self.MoveSpeed_Sec`) (* (`GameplayStatics.GetWorldDeltaSeconds`) 2.0))))))

(fn `MoveToPlayer`
  (`self.MoveToDestinationPos` (`self.K2_GetActorLocation` (`GameplayStatics.GetPlayerPawn` 0)) true)
  (bind _fin (`self.SecCnt` 5.0))
  (set `self.FinActionFlag` (or _fin (`self.FitlyDistanseFlag`))))

(fn `NoShowWidget`
  (`Widget.RemoveFromParent` (`self.HPBarWidget`)))

(fn `Rotate to Face Player`
  (bind _returnvalue (`self.GetActorForwardVector`))
  (bind _toplayervector (`self.ToPlayerVector`))
  (bind _returnvalue_2 (`KismetMathLibrary.RotateAngleAxis` _returnvalue (* (`self.RotateSpeed_Sec`) (`GameplayStatics.GetWorldDeltaSeconds`)) (`KismetMathLibrary.Cross_VectorVector` (`self.GetActorForwardVector`) _toplayervector)))
  (if (>= (`KismetMathLibrary.Dot_VectorVector` _returnvalue_2 _returnvalue) (`KismetMathLibrary.Dot_VectorVector` _returnvalue _toplayervector))
    (`self.K2_SetActorRotation` (`KismetMathLibrary.Conv_VectorToRotator` _returnvalue_2))
    (else
      (`self.K2_SetActorRotation` (`KismetMathLibrary.Conv_VectorToRotator` (`self.ToPlayerVector`))))))

(fn `Rotate To Face Player XY plane`
  (locals (ToPlayerVecInXYPlane :type "Vector2D Structure") (SelfForwardVecInXYPlane :type "Vector2D Structure"))
  (bind (_returnvalue_roll _returnvalue_pitch) (`KismetMathLibrary.BreakRotator` (`self.K2_GetActorRotation`)))
  (bind (_returnvalue_roll_2 _returnvalue_pitch_2 _returnvalue_yaw) (`KismetMathLibrary.BreakRotator` (`KismetMathLibrary.Conv_VectorToRotator` (`self.ToPlayerVector`))))
  (bind _output_get (set `local.ToPlayerVecInXYPlane` (`KismetMathLibrary.Normal2D` (`KismetMathLibrary.Conv_VectorToVector2D` (`self.ToPlayerVector`)))))
  (bind _output_get_2 (set `local.SelfForwardVecInXYPlane` (`KismetMathLibrary.Normal2D` (`KismetMathLibrary.Conv_VectorToVector2D` (`self.GetActorForwardVector`)))))
  (bind _returnvalue (`KismetMathLibrary.Conv_Vector2DToVector` _output_get_2))
  (bind _returnvalue_2 (`KismetMathLibrary.Conv_Vector2DToVector` _output_get))
  (bind _returnvalue_3 (`KismetMathLibrary.RotateAngleAxis` _returnvalue (* (`self.RotateSpeed_Sec`) (`GameplayStatics.GetWorldDeltaSeconds`)) (`KismetMathLibrary.Cross_VectorVector` _returnvalue _returnvalue_2)))
  (if (>= (`KismetMathLibrary.Dot_VectorVector` _returnvalue_3 _returnvalue) (`KismetMathLibrary.Dot_VectorVector` _returnvalue _returnvalue_2))
    (bind (_returnvalue_roll_3 _returnvalue_pitch_3 _returnvalue_yaw_2) (`KismetMathLibrary.BreakRotator` (`KismetMathLibrary.Conv_VectorToRotator` _returnvalue_3)))
    (`self.K2_SetActorRotation` (`KismetMathLibrary.MakeRotator` _returnvalue_roll _returnvalue_pitch _returnvalue_yaw_2))
    (else
      (`self.K2_SetActorRotation` (`KismetMathLibrary.MakeRotator` _returnvalue_roll _returnvalue_pitch _returnvalue_yaw)))))

(fn `Rotate To Face XZ Plane`
  (`self.K2_SetActorRotation` (`KismetMathLibrary.MakeRotator` 0.0)))

(fn `RotateToDestinationPos`
  (params (DestinationPos :type "Vector Structure"))
  (locals (ToDestinationVec :type "Vector Structure"))
  (bind _returnvalue (`self.GetActorForwardVector`))
  (bind _output_get (set `local.ToDestinationVec` (`KismetMathLibrary.Normal` (- DestinationPos (`self.K2_GetActorLocation`)))))
  (bind _returnvalue_2 (`KismetMathLibrary.RotateAngleAxis` _returnvalue (* (`self.RotateSpeed_Sec`) (`GameplayStatics.GetWorldDeltaSeconds`)) (`KismetMathLibrary.Cross_VectorVector` (`self.GetActorForwardVector`) _output_get)))
  (if (>= (`KismetMathLibrary.Dot_VectorVector` _returnvalue_2 _returnvalue) (`KismetMathLibrary.Dot_VectorVector` _returnvalue _output_get))
    (`self.K2_SetActorRotation` (`KismetMathLibrary.Conv_VectorToRotator` _returnvalue_2))
    (else
      (`self.K2_SetActorRotation` (`KismetMathLibrary.Conv_VectorToRotator` _output_get)))))

(fn `RotateToPosXYPlane`
  (params (DestinationPos :type "Vector Structure"))
  (locals (ToDestinationPosVecInXYPlane :type "Vector2D Structure") (SelfForwardVecInXYPlane :type "Vector2D Structure"))
  (bind (_returnvalue_roll _returnvalue_pitch) (`KismetMathLibrary.BreakRotator` (`self.K2_GetActorRotation`)))
  (bind _returnvalue (`KismetMathLibrary.Normal2D` (`KismetMathLibrary.Conv_VectorToVector2D` (`KismetMathLibrary.Normal` (- DestinationPos (`self.K2_GetActorLocation`))))))
  (bind (_returnvalue_roll_2 _returnvalue_pitch_2 _returnvalue_yaw) (`KismetMathLibrary.BreakRotator` (`KismetMathLibrary.Conv_VectorToRotator` (`KismetMathLibrary.Conv_Vector2DToVector` _returnvalue))))
  (bind _output_get (set `local.ToDestinationPosVecInXYPlane` _returnvalue))
  (bind _output_get_2 (set `local.SelfForwardVecInXYPlane` (`KismetMathLibrary.Normal2D` (`KismetMathLibrary.Conv_VectorToVector2D` (`self.GetActorForwardVector`)))))
  (bind _returnvalue_2 (`KismetMathLibrary.Conv_Vector2DToVector` _output_get_2))
  (bind _returnvalue_3 (`KismetMathLibrary.Conv_Vector2DToVector` _output_get))
  (bind _returnvalue_4 (`KismetMathLibrary.RotateAngleAxis` _returnvalue_2 (* (`self.RotateSpeed_Sec`) (`GameplayStatics.GetWorldDeltaSeconds`)) (`KismetMathLibrary.Cross_VectorVector` _returnvalue_2 _returnvalue_3)))
  (if (>= (`KismetMathLibrary.Dot_VectorVector` _returnvalue_4 _returnvalue_2) (`KismetMathLibrary.Dot_VectorVector` _returnvalue_2 _returnvalue_3))
    (bind (_returnvalue_roll_3 _returnvalue_pitch_3 _returnvalue_yaw_2) (`KismetMathLibrary.BreakRotator` (`KismetMathLibrary.Conv_VectorToRotator` _returnvalue_4)))
    (`self.K2_SetActorRotation` (`KismetMathLibrary.MakeRotator` _returnvalue_roll _returnvalue_pitch _returnvalue_yaw_2))
    (else
      (`self.K2_SetActorRotation` (`KismetMathLibrary.MakeRotator` _returnvalue_roll _returnvalue_pitch _returnvalue_yaw)))))

(fn `Rush Base`
  (params (DecelerationFlag :type Boolean))
  (bind _rushspeed (`self.RushSpeed`))
  (bind _returnvalue (- (`self.NowSpeed`) (* (* (`GameplayStatics.GetWorldDeltaSeconds`) 2.0) (`self.RushDeacceleration`))))
  (bind _returnvalue_2 (+ (`self.NowSpeed`) (* (* (`GameplayStatics.GetWorldDeltaSeconds`) 2.0) (`self.RushAcceleration`))))
  (if DecelerationFlag
    (if (> (`self.NowSpeed`) 0.0)
      (if (> _returnvalue 0.0)
        (set `self.NowSpeed` _returnvalue)
        (else
          (set `self.NowSpeed` 0.0)))
      (bind (_sweephitresult _returnvalue_3) (`self.K2_SetActorLocation` (+ (`self.K2_GetActorLocation`) (* (`self.RushVector`) (* (`self.NowSpeed`) (* (`GameplayStatics.GetWorldDeltaSeconds`) 2.0)))) true :!label _label))
      (if (not _returnvalue_3)
        (set `self.FinActionFlag` true)
        (set `self.ATK` 0.0)))
    (elif (< (`self.NowSpeed`) (`self.RushSpeed`))
      (if (< _returnvalue_2 _rushspeed)
        (set `self.NowSpeed` _returnvalue_2)
        (goto _label)
        (else
          (set `self.NowSpeed` _rushspeed)
          (goto _label)))
      (else
        (goto _label)))))

(fn `SecCnt`
  (params (SetSec :type "Float (double-precision)"))
  (returns (Fin :type Boolean) (NowSec :type "Float (double-precision)"))
  (bind _output_get (set `self.TimeCnt` (+ (`self.TimeCnt`) (* (`GameplayStatics.GetWorldDeltaSeconds`) 2.0))))
  (if (> _output_get SetSec)
    (set `self.TimeCnt` 0.0)
    (return true _output_get)
    (else
      (return false _output_get))))

(fn `UserConstructionScript`)