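; BP_WaterBreath is an enemy water breath attack that damages the player on contact.
; StartBreath turns on the particle spawn rate and begins a timer, and the capsule becomes query-only collision after a short delay so damage lags the visual.
; Overlapping actors tagged Player receive SetDamage with no knockback force.
; When the breath duration elapses, StopBreath cuts the particles, disables collision and clears the flag, as it also does on BeginPlay.
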(event `self.ReceiveBeginPlay`
  (`self.StopBreath`))

(event `self.ReceiveTick`
  (params (DeltaSeconds :type "Float (single-precision)"))
  (if (`self.BreathFlag`)
    (bind _output_get (set `self.BreathSec_Cnt` (+ (`self.BreathSec_Cnt`) (`GameplayStatics.GetWorldDeltaSeconds`))))
    (if (>= _output_get (`self.BreathSec`))
      (`self.StopBreath`)
      (set `self.BreathSec_Cnt` 0.0)
      (elif (>= _output_get 0.25)
        (`PrimitiveComponent.SetCollisionEnabled` (`self.Capsule`) "QueryOnly")))))

(event `self.Capsule.OnComponentBeginOverlap`
  (params (OverlappedComponent :type "PrimitiveComponent Object Reference") (OtherActor :type "Actor Object Reference") (OtherComp :type "PrimitiveComponent Object Reference") (OtherBodyIndex :type Integer) (bFromSweep :type Boolean) (SweepResult :type "HitResult Structure (by ref)"))
  (if (`self.ActorHasTag` OtherActor "Player")
    (bind _asplayer_base (cast `PlayerBase` OtherActor))
    (`PlayerBase.SetDamage` _asplayer_base (`self.Attack Num`) (0.0 0.0 0.0) 0.0)))

(fn `StartBreath`
  (`FXSystemComponent.SetFloatParameter` (`self.PT_WaterBreath`) "SpawnRate" 1.0)
  (set `self.BreathFlag` true))

(fn `StopBreath`
  (`FXSystemComponent.SetFloatParameter` (`self.PT_WaterBreath`) "SpawnRate" 0.0)
  (`PrimitiveComponent.SetCollisionEnabled` (`self.Capsule`) "NoCollision")
  (set `self.BreathFlag` false))

(fn `UserConstructionScript`)