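; BP_ThreadBullet is an enemy projectile, apparently a thread shot, that damages the player on contact.
; Tick moves it along MoveVec at Speed using doubled delta time, after an optional one-frame hold from StayFlag, until LifeSec elapses.
; Collision overlaps skip "Enemyr"-tagged actors, apply ATK through PlayerBase SetDamage to players, and end life on other hits.
; Clearing LifeFlag defers destruction to a later Tick.
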(event `self.ReceiveTick`
  (params (DeltaSeconds :type "Float (single-precision)"))
  (if (`self.StayFlag`)
    (set `self.SecCntNum` (+ (* (`GameplayStatics.GetWorldDeltaSeconds`) 2.0) (`self.SecCntNum`)))
    (set `self.StayFlag` false)
    (elif (`self.LifeFlag`)
      (`self.K2_SetActorLocation` (+ (`self.K2_GetActorLocation`) (* (`self.MoveVec`) (* (`self.Speed`) (* (`GameplayStatics.GetWorldDeltaSeconds`) 2.0)))))
      (bind _output_get (set `self.SecCntNum` (+ (* (`GameplayStatics.GetWorldDeltaSeconds`) 2.0) (`self.SecCntNum`))))
      (if (> _output_get (`self.LifeSec`))
        (set `self.LifeFlag` false))
      (else
        (`self.K2_DestroyActor`)))))

(event `self.Collision.OnComponentBeginOverlap`
  (params (OverlappedComponent :type "PrimitiveComponent Object Reference") (OtherActor :type "Actor Object Reference") (OtherComp :type "PrimitiveComponent Object Reference") (OtherBodyIndex :type Integer) (bFromSweep :type Boolean) (SweepResult :type "HitResult Structure (by ref)"))
  (if (not (`self.ActorHasTag` OtherActor "Enemyr"))
    (if (`self.ActorHasTag` OtherActor "Player")
      (bind _asplayer_base (cast `PlayerBase` OtherActor))
      (`PlayerBase.SetDamage` _asplayer_base (`self.ATK`) (0.0 0.0 0.0) 0.0))
    (set `self.LifeFlag` false)))

(fn `UserConstructionScript`)