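; Spider enemy that chases the player, shoots thread bullets and performs a jumping press attack, with tuning loaded from DT_SpiderStatus.
; Each action is a timed, flag-driven state function; FinAction resets state and asks BP_SpiderAI to select the next.
; The press uses hand-integrated motion, reaching the clamped player position at apex, hovering, then sweeping down with damage active until blocked.
; Death fades the material and aura before destroying both components.
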(event `self.ReceiveBeginPlay`
  (bind _pt_enemyaura (`self.PT_EnemyAura`))
  (`|ExecutionSequence`
    (:`then_0`
      (`FXSystemComponent.SetActorParameter` _pt_enemyaura "VertSurfaceActor" self)
      (`SceneComponent.SetRelativeScale3D` _pt_enemyaura (0.125 0.125 0.2))
      (`FXSystemComponent.SetFloatParameter` _pt_enemyaura "SpawnRate" 0.0))
    (:`then_1`
      (`self.FinAction`)
      (bind _returnvalue (`|GetDataTableRow` "/Game/Main/DataTable/DT_SpiderStatus.DT_SpiderStatus" "SpiderStatus")
        (:`then`
          (set `self.PressPrepareSec` (break `/Game/Main/BP/Enemy/Spider/ST_SpiderStatus` _returnvalue))
          (set `self.PressStayAirSec` (`.PressStayAirSec_9_CBFB344D40FDEF90EFCF27AF20CBE77D` (break `/Game/Main/BP/Enemy/Spider/ST_SpiderStatus` _returnvalue)))
          (set `self.PressAfterSec` (`.PressAfterSec_13_5743A8E143E15A054A047EBF81927146` (break `/Game/Main/BP/Enemy/Spider/ST_SpiderStatus` _returnvalue)))
          (set `self.ForJumpGravity` (`.ForJumpGravity_19_261F17854FAF0916A1F85E8DFA05B5BB` (break `/Game/Main/BP/Enemy/Spider/ST_SpiderStatus` _returnvalue)))
          (set `self.ForFallGravity` (`.ForFallGravity_20_2DB9B72347C4373883A89BB51184B18A` (break `/Game/Main/BP/Enemy/Spider/ST_SpiderStatus` _returnvalue)))
          (set `self.JumpPower` (`.JumpPower_21_E9D0D14849FA6D99DD40429F4DBEBC96` (break `/Game/Main/BP/Enemy/Spider/ST_SpiderStatus` _returnvalue)))
          (set `self.MaxJumpDistance` (`.MaxJumpDistance_23_B00DC8F640B27B9B5FB81D8229DAF56A` (break `/Game/Main/BP/Enemy/Spider/ST_SpiderStatus` _returnvalue)))
          (set `self.PressAttackNum` (`.PressAttackNum_28_ACBD883C42E796FB862CB482AAF6DE9E` (break `/Game/Main/BP/Enemy/Spider/ST_SpiderStatus` _returnvalue)))
          (set `self.ThreadBulletPrepareSec` (`.ThreadBulletPrepareSec_29_BCEF53944715BF16EFBFEE903B3E8D3C` (break `/Game/Main/BP/Enemy/Spider/ST_SpiderStatus` _returnvalue)))
          (set `self.ThreadBulletAfterSec` (`.ThreadBulletAfterSec_30_B873F173486F98E784017A9C08C5F835` (break `/Game/Main/BP/Enemy/Spider/ST_SpiderStatus` _returnvalue)))
          (set `self.ThreadBulletAttackNum` (`.ThreadBulletAttackNum_32_5F238CAB44B17ABB71A9EFB86704C12E` (break `/Game/Main/BP/Enemy/Spider/ST_SpiderStatus` _returnvalue)))
          (set `self.ThreadBulletSpeed` (`.ThreadBulletSpeed_34_F32FFE0B48C8024D40FB319A639E409A` (break `/Game/Main/BP/Enemy/Spider/ST_SpiderStatus` _returnvalue)))
          (set `self.ThreadBulletLifeSec` (`.ThreadBulletLifeSec_36_6DA7317049C4824F1DD267A99017928D` (break `/Game/Main/BP/Enemy/Spider/ST_SpiderStatus` _returnvalue)))
          (`parent.ReceiveBeginPlay`))))))

(event `self.ReceiveTick`
  (params (DeltaSeconds :type "Float (single-precision)"))
  (`parent.ReceiveTick` DeltaSeconds))

(fn `Fall`
  (bind (_sweephitresult _returnvalue) (`self.K2_SetActorLocation` (+ (`self.K2_GetActorLocation`) (* (* (`self.GetActorUpVector`) -1.0) (* (`self.NowPressFallSpeed`) (* (`GameplayStatics.GetWorldDeltaSeconds`) 2.0)))) true))
  (if _returnvalue
    (set `self.NowPressFallSpeed` (+ (`self.NowPressFallSpeed`) (* (`self.ForFallGravity`) (* (`GameplayStatics.GetWorldDeltaSeconds`) 2.0))))
    (else
      (set `self.NowPressFallSpeed` 0.0)
      (set `self.FinActionFlag` true))))

(fn `FinAction`
  (bind _asbp_spider_ai (cast `/Game/Main/BP/Enemy/Spider/BP_SpiderAI` (`AIBlueprintHelperLibrary.GetAIController` self)))
  (`/Game/Main/BP/Enemy/Spider/BP_SpiderAI.SelectAction` _asbp_spider_ai)
  (set `self.AttackStartedFlag` false)
  (set `self.FinActionFlag` false)
  (set `self.StayAirFlag` false)
  (set `self.FallFlag` false)
  (set `self.playStandUpAnimFlag` false)
  (set `self.TimeCnt` 0.0))

(fn `Jump`
  (locals (NewLocalVar_0 :type "Float (double-precision)"))
  (if (== (`self.NowJumpPower`) 0.0)
    (set `self.NowJumpPower` (`self.JumpPower`)))
  (`self.K2_SetActorLocation` (+ (`self.K2_GetActorLocation`) (* (`self.GetActorUpVector`) (* (`self.NowJumpPower`) (* (`GameplayStatics.GetWorldDeltaSeconds`) 2.0)))))
  (set `self.NowJumpPower` (- (`self.NowJumpPower`) (* (`self.ForJumpGravity`) (* (`GameplayStatics.GetWorldDeltaSeconds`) 2.0))))
  (if (<= (`self.NowJumpPower`) 0.0)
    (set `self.NowJumpPower` 0.0)
    (set `self.StayAirFlag` true)))

(fn `JumpXYMove`
  (`self.K2_SetActorLocation` (+ (`self.K2_GetActorLocation`) (* (`self.GetActorForwardVector`) (* (`self.JumpXYSpeed`) (* (`GameplayStatics.GetWorldDeltaSeconds`) 2.0))))))

(fn `MoveToPlayerSpider`
  (if (`self.FinActionFlag`)
    (`self.FinAction`)
    (else
      (`self.MoveToPlayer`))))

(fn `PressAttack`
  (bind _pressaftersec (`self.PressAfterSec`))
  (if (`self.AttackStartedFlag`)
    (if (`self.StayAirFlag`)
      (if (`self.FallFlag`)
        (if (`self.FinActionFlag`)
          (set `self.ATK` 0.0)
          (set `self.NowPressFallSpeed` 0.0)
          (bind (_fin _nowsec) (`self.SecCnt` _pressaftersec))
          (if (<= (- _pressaftersec _nowsec) 1.0)
            (set `self.playStandUpAnimFlag` true))
          (if _fin
            (`self.FinAction`))
          (else
            (`self.Fall`)))
        (else
          ;[1 1 1] 滞空
          (bind _fin_2 (`self.SecCnt` (`self.PressStayAirSec`)))
          (if _fin_2
            (set `self.FallFlag` true)
            (set `self.ATK` (`self.PressAttackNum`)))))
      (else
        (`self.JumpXYMove`)
        (`self.Jump`)))
    (else
      (`self.PressPrepare`))))

(fn `PressPrepare`
  (bind _returnvalue (`self.K2_GetActorLocation`))
  (`self.Rotate To Face Player XY plane`)
  (bind _fin (`self.SecCnt` (`self.PressPrepareSec`)))
  (if _fin
    (set `self.AttackStartedFlag` true)
    (if (> (`self.MaxJumpDistance`) (`self.Distance to Player`))
      (bind _output_get (set `self.JumpDestinationPos` (`KismetMathLibrary.Conv_VectorToVector2D` (`self.K2_GetActorLocation` (`GameplayStatics.GetPlayerPawn` 0)))))
      (set `self.JumpDistance` (`KismetMathLibrary.VSize` (`KismetMathLibrary.Conv_Vector2DToVector` (- _output_get (`KismetMathLibrary.Conv_VectorToVector2D` (`self.K2_GetActorLocation`))))))
      (else
        (bind _output_get_2 (set `self.JumpDestinationPos` (`KismetMathLibrary.Conv_VectorToVector2D` (+ _returnvalue (* (`self.ToPlayerVector`) (`self.MaxJumpDistance`))))))
        (set `self.JumpDistance` (`KismetMathLibrary.VSize` (`KismetMathLibrary.Conv_Vector2DToVector` (- _output_get_2 (`KismetMathLibrary.Conv_VectorToVector2D` _returnvalue)))))))
    (set `self.JumpXYSpeed` (/ (`self.JumpDistance`) (/ (`self.JumpPower`) (`self.ForJumpGravity`))))))

(fn `Shot Thread Bullet`
  (bind (_returnvalue_location _returnvalue_rotation) (`KismetMathLibrary.BreakTransform` (`self.GetTransform`)))
  (if (`self.AttackStartedFlag`)
    (bind _fin (`self.SecCnt` (`self.ThreadBulletAfterSec`)))
    (if _fin
      (`self.FinAction`))
    (else
      (`self.Rotate To Face Player XY plane`)
      (bind _fin_2 (`self.SecCnt` (`self.ThreadBulletPrepareSec`)))
      (if _fin_2
        (bind _returnvalue (`|SpawnActorFromClass` "/Game/Main/BP/Enemy/BP_ThreadBullet.BP_ThreadBullet_C" (`KismetMathLibrary.ComposeTransforms` (`KismetMathLibrary.Conv_VectorToTransform` (`self.ThreadBulletSpawnPos`)) (`KismetMathLibrary.MakeTransform` _returnvalue_location _returnvalue_rotation)) "Undefined" "OverrideRootScale" null null))
        (set `/Game/Main/BP/Enemy/BP_ThreadBullet.ATK` (`self.ThreadBulletAttackNum`) _returnvalue)
        (set `/Game/Main/BP/Enemy/BP_ThreadBullet.MoveVec` (`self.GetActorForwardVector`) _returnvalue)
        (set `/Game/Main/BP/Enemy/BP_ThreadBullet.Speed` (`self.ThreadBulletSpeed`) _returnvalue)
        (set `/Game/Main/BP/Enemy/BP_ThreadBullet.LifeSec` (`self.ThreadBulletLifeSec`) _returnvalue)
        (set `self.AttackStartedFlag` true)
        (set `self.FinActionFlag` true)))))

(fn `SpiderDead`
  (bind _spider_model (`self.Spider_model`))
  (bind (_fin _nowsec) (`self.SecCnt` (`self.DeadDirectingSec`)))
  (if _fin
    (`ActorComponent.K2_DestroyComponent` _spider_model)
    (`ActorComponent.K2_DestroyComponent` (`self.PT_EnemyAura`))
    (else
      (bind _returnvalue (`PrimitiveComponent.CreateDynamicMaterialInstance` _spider_model 0 "/Game/Main/Meshes/Enemy/Carp/lambert3_Dead.lambert3_Dead" "None"))
      (bind _returnvalue_2 (/ (- (`self.DeadDirectingSec`) _nowsec) (`self.DeadDirectingSec`)))
      (`MaterialInstanceDynamic.SetScalarParameterValue` _returnvalue "Opacity" _returnvalue_2)
      (`FXSystemComponent.SetFloatParameter` (`self.PT_EnemyAura`) "SpawnRate" _returnvalue_2))))

(fn `UserConstructionScript`
  (`parent.UserConstructionScript`))