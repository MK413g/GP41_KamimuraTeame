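; AI controller for the spider enemy that picks its action and runs its behavior tree.
; On BeginPlay it calls SelectAction, then starts BT_SpiderAI.
; SelectAction maps the controlled BP_EnemyBase pawn's player-distance state to a spider action, fixed at short range and random between two at middle range.
; At long range it also picks randomly between two, except that the third action is always followed by the second.
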(event `self.ReceiveBeginPlay`
  (`self.SelectAction`)
  (`self.RunBehaviorTree` "/Game/Main/BP/Enemy/Spider/BT_SpiderAI.BT_SpiderAI"))

(fn `SelectAction`
  (bind _asbp_enemy_base (cast `/Game/Main/BP/Enemy/EnemyBase/BP_EnemyBase` (`self.K2_GetPawn`)))
  (switch `/Game/Main/BP/Enemy/EnemyBase/DISTANCE_STATE` (`/Game/Main/BP/Enemy/EnemyBase/BP_EnemyBase.TO_PLAYER_DISTANSE_STATE` _asbp_enemy_base)
    (:`NewEnumerator0`
      (set `self.SELECTED_ACTION` "NewEnumerator0"))
    (:`NewEnumerator1`
      (set `self.SELECTED_ACTION` (cast `/Game/Main/BP/Enemy/Spider/SPIDER_ACTION` (`KismetMathLibrary.Conv_IntToByte` (`KismetMathLibrary.RandomInteger` 2)))))
    (:`NewEnumerator2`
      (if (`|EnumEquality` (`self.SELECTED_ACTION`) "NewEnumerator2")
        (set `self.SELECTED_ACTION` "NewEnumerator1")
        (else
          (set `self.SELECTED_ACTION` (cast `/Game/Main/BP/Enemy/Spider/SPIDER_ACTION` (`KismetMathLibrary.Conv_IntToByte` (+ (`KismetMathLibrary.RandomInteger` 2) 1)))))))))

(fn `UserConstructionScript`
  (`parent.UserConstructionScript`))