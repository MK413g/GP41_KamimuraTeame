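; Carp (koi) enemy that rushes the player or fires a water-breath laser, with stats loaded from DT_CarpStatus.
; Timed action functions step through prepare, attack and recovery using flags and SecCnt, then FinAction has BP_CarpAI select the next action.
; Rush arms contact damage via ATK on mesh hits, while water breath spawns BP_LaserCopy.
; Flinch delegates to the parent, and death fades materials and aura before destroying those components.
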(event `self.ReceiveBeginPlay`
  (bind _pt_enemyaura (`self.PT_EnemyAura`))
  (`|ExecutionSequence`
    (:`then_0`
      (`FXSystemComponent.SetActorParameter` _pt_enemyaura "VertSurfaceActor" self)
      (`SceneComponent.SetRelativeScale3D` _pt_enemyaura (0.1 0.5 0.4))
      (`FXSystemComponent.SetFloatParameter` _pt_enemyaura "SpawnRate" 0.0))
    (:`then_1`
      (`self.FinAction`)
      (bind _returnvalue (`|GetDataTableRow` "/Game/Main/DataTable/DT_CarpStatus.DT_CarpStatus" "CarpStatus")
        (:`then`
          (set `self.HP` (break `/Game/Main/BP/Enemy/Carp/ST_CarpState` _returnvalue))
          (set `self.MoveSpeed_Sec` (`.MoveSpeed_38_D2B7BE2D4875D1C1D3BB479A2B5DA3E0` (break `/Game/Main/BP/Enemy/Carp/ST_CarpState` _returnvalue)))
          (set `self.RotateSpeed_Sec` (`.RotateSpeed_37_3CB5073D49250B92406A308753F0C366` (break `/Game/Main/BP/Enemy/Carp/ST_CarpState` _returnvalue)))
          (set `self.RushSpeed` (`.RushSpeed_36_0739916243CFA30A1E13DAA08C76ECE9` (break `/Game/Main/BP/Enemy/Carp/ST_CarpState` _returnvalue)))
          (set `self.RushPrepareSec` (`.RushPrepareSec_18_16776D5645EAB20195AB3BB6786874AD` (break `/Game/Main/BP/Enemy/Carp/ST_CarpState` _returnvalue)))
          (set `self.RushSec` (`.RushSec_11_AB02E68548097F459979089B3829EDCE` (break `/Game/Main/BP/Enemy/Carp/ST_CarpState` _returnvalue)))
          (set `self.RushAfterSec` (`.AfterRushSec_17_7BBDDE1147BF97109E0DA0BB10737B88` (break `/Game/Main/BP/Enemy/Carp/ST_CarpState` _returnvalue)))
          (set `self.RushAttackNum` (`.RushAttackNum_19_BC100696497CE9C4D28956A2CAC31D15` (break `/Game/Main/BP/Enemy/Carp/ST_CarpState` _returnvalue)))
          (set `self.WaterBreathPrepareSec` (`.WaterBreathPrepareSec_23_B4D154714D4A676881844B932A02697E` (break `/Game/Main/BP/Enemy/Carp/ST_CarpState` _returnvalue)))
          (set `self.WaterBreathSec` (`.WaterBreathShotSec_29_9132FF5643AC4B5C9B5E35A537AC9DF9` (break `/Game/Main/BP/Enemy/Carp/ST_CarpState` _returnvalue)))
          (set `self.WaterBreathAfterSec` (`.AfterWaterBreathSec_30_432902DB48D0ABDA1477718E0DE2E103` (break `/Game/Main/BP/Enemy/Carp/ST_CarpState` _returnvalue)))
          (set `self.WaterBreathAttackNum` (`.WaterBreathAttackNum_21_DFAE1E66452F11444087469E4F98AD59` (break `/Game/Main/BP/Enemy/Carp/ST_CarpState` _returnvalue)))
          (set `self.FlinchSec` (`.FlinchSec_47_AE8FC292422866C00DA29CB50AE29462` (break `/Game/Main/BP/Enemy/Carp/ST_CarpState` _returnvalue)))
          (set `self.BeFlinchDamage` (`.FlinchHitNum_50_586F5D2C4176BC657F9D9CA93F9AF677` (break `/Game/Main/BP/Enemy/Carp/ST_CarpState` _returnvalue)))
          (`parent.ReceiveBeginPlay`))))))

(event `self.ReceiveActorBeginOverlap`
  (params (OtherActor :type "Actor Object Reference")))

(event `self.ReceiveTick`
  (params (DeltaSeconds :type "Float (single-precision)"))
  (`parent.ReceiveTick` DeltaSeconds))

(event `self.3D_koi.OnComponentHit`
  (params (HitComponent :type "PrimitiveComponent Object Reference") (OtherActor :type "Actor Object Reference") (OtherComp :type "PrimitiveComponent Object Reference") (NormalImpulse :type "Vector Structure") (Hit :type "HitResult Structure (by ref)"))
  (bind _atk (`self.ATK`))
  (if (`self.ActorHasTag` OtherActor "Player")
    (bind _asbp_player (cast `/Game/Main/BP/Player/BP_Player` OtherActor))
    (if (> _atk 0.0)
      (`PlayerBase.SetDamage` _asbp_player _atk (0.0 0.0 0.0) 0.0))))

(fn `CarpDead`
  (bind _3d_koi (`self.3D_koi`))
  (if (not (`self.FinDeadDirectingFlag`))
    (bind (_fin _nowsec) (`self.SecCnt` (`self.DeadDirectingSec`)))
    (if _fin
      (`ActorComponent.K2_DestroyComponent` (`self.3D_koi`))
      (`ActorComponent.K2_DestroyComponent` (`self.PT_EnemyAura`))
      (set `self.FinDeadDirectingFlag` true)
      (else
        (bind _returnvalue (`PrimitiveComponent.CreateDynamicMaterialInstance` _3d_koi 0 "/Game/Main/Meshes/Enemy/Carp/lambert3_Dead.lambert3_Dead" "None"))
        (bind _returnvalue_2 (/ (- (`self.DeadDirectingSec`) _nowsec) (`self.DeadDirectingSec`)))
        (`MaterialInstanceDynamic.SetScalarParameterValue` _returnvalue "Opacity" _returnvalue_2)
        (bind _returnvalue_3 (`PrimitiveComponent.CreateDynamicMaterialInstance` _3d_koi 1 "/Game/Main/Meshes/Enemy/Carp/lambert4_C_dead.lambert4_C_dead" "None"))
        (`MaterialInstanceDynamic.SetScalarParameterValue` _returnvalue_3 "Opacity" _returnvalue_2)
        (`FXSystemComponent.SetFloatParameter` (`self.PT_EnemyAura`) "SpawnRate" _returnvalue_2)))))

(fn `CarpFlinch`
  (`parent.Flinch`)
  (if (not (`self.FlinchFlag`))
    (`self.FinAction`)
    (set `self.FlinchFlag` false)))

(fn `CarpRush`
  (if (`self.AttackStartedFlag`)
    (if (`self.FinActionFlag`)
      (set `self.ATK` 0.0)
      (`self.Rush Base` true)
      (bind _fin (`self.SecCnt` (`self.RushAfterSec`)))
      (if _fin
        (`self.FinAction`))
      (else
        (`self.Rush Base` false)
        (bind _fin_2 (`self.SecCnt` (`self.RushSec`)))
        (if _fin_2
          (set `self.FinActionFlag` true)
          (set `self.ATK` 0.0))))
    (else
      ;[1 1 1] 方向決定
      (`self.Rotate To Face Player XY plane`)
      (bind _fin_3 (`self.SecCnt` (`self.RushPrepareSec`)))
      (if _fin_3
        (set `self.ATK` (`self.RushAttackNum`))
        (set `self.RushVector` (`self.GetActorForwardVector`))
        (set `self.AttackStartedFlag` true)
        (`SoundManagerBase.PlaySoundLocation` "/Game/Main/Sound/SE/Enemey/SE_Rush.SE_Rush" "SE" (`self.K2_GetActorLocation`) 1.0 1.0 0.0 null null)))))

(fn `FinAction`
  (bind _asbp_carp_ai (cast `/Game/Main/BP/Enemy/Carp/BP_CarpAI` (`self.GetController`)))
  (`/Game/Main/BP/Enemy/Carp/BP_CarpAI.Select Next Action` _asbp_carp_ai)
  (`|ExecutionSequence`
    (:`then_0`
      (set `self.AttackStartedFlag` false)
      (set `self.FinActionFlag` false)
      (set `self.StartPlayBreathPrepareAnimFlag` false))
    (:`then_1`
      (set `self.AttackMotionFlag` (not (`|EnumEquality` (`/Game/Main/BP/Enemy/Carp/BP_CarpAI.SELECTED_CARP_ACTION` _asbp_carp_ai) "NewEnumerator2"))))))

(fn `Move To Player Carp`
  (if (`self.FinActionFlag`)
    (`self.FinAction`)
    (else
      (`self.MoveToPlayer`))))

(fn `UserConstructionScript`
  (`parent.UserConstructionScript`))

(fn `WaterBreath`
  (bind (_returnvalue_location _returnvalue_rotation) (`KismetMathLibrary.BreakTransform` (`self.GetTransform`)))
  (if (`self.AttackStartedFlag`)
    (if (`self.FinActionFlag`)
      (bind _fin (`self.SecCnt` (`self.WaterBreathAfterSec`)))
      (`self.Rotate To Face Bace XZ Plane`)
      (if _fin
        (`self.FinAction`)
        (set `self.StartPlayBreathPrepareAnimFlag` false))
      (else
        (bind _fin_2 (`self.SecCnt` (`self.WaterBreathSec`)))
        (set `self.FinActionFlag` _fin_2)))
    (else
      ;[1 1 1] 方向決定
      (`self.Rotate to Face Player`)
      (bind (_fin_3 _nowsec) (`self.SecCnt` (`self.WaterBreathPrepareSec`)))
      (set `self.StartPlayBreathPrepareAnimFlag` (> _nowsec (- (`self.WaterBreathPrepareSec`) (`self.PlayBreathPrepareAnimSec`))))
      (if _fin_3
        (set `self.RushVector` (`self.GetActorForwardVector`))
        (set `self.AttackStartedFlag` true)
        (bind _returnvalue (`|SpawnActorFromClass` "/Game/Main/BP/Enemy/BP_LaserCopy.BP_LaserCopy_C" (`KismetMathLibrary.ComposeTransforms` (`KismetMathLibrary.Conv_VectorToTransform` (`self.WaterBreathSpawnPos`)) (`KismetMathLibrary.MakeTransform` _returnvalue_location _returnvalue_rotation)) "Undefined" "OverrideRootScale" null null))
        (`self.SetActorScale3D` _returnvalue (/ (`self.GetActorScale3D` _returnvalue) (10.0 2.0 2.5)))
        (set `/Game/Main/BP/Enemy/BP_LaserCopy.Damage` (`self.WaterBreathAttackNum`) _returnvalue)
        (set `/Game/Main/BP/Enemy/BP_LaserCopy.ShotSec` (`self.WaterBreathSec`) _returnvalue)))))