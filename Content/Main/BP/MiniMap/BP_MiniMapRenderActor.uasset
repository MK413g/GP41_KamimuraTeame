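; Minimap render actor that shows a material on a plane and can follow an enemy's position.
; On BeginPlay it applies its material to the plane and stores the actor returned by a single BP_EnemyBase class lookup as its target.
; While IsTarget is set and that target is valid, Tick moves the root component to the target's world location.
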(event `self.ReceiveBeginPlay`
  (`PrimitiveComponent.SetMaterial` (`self.Plane`) 0 (`self.Material`))
  (bind _returnvalue (`GameplayStatics.GetActorOfClass` "/Game/Main/BP/Enemy/EnemyBase/BP_EnemyBase.BP_EnemyBase_C"))
  (`/Engine/EditorBlueprintResources/StandardMacros.IsValid` _returnvalue
    (:`Is Valid`
      (set `self.TargetActor` _returnvalue))))

(event `self.ReceiveTick`
  (params (DeltaSeconds :type "Float (single-precision)"))
  (if (and (`self.isTarget`) (`KismetSystemLibrary.IsValid` (`self.TargetActor`)))
    (`SceneComponent.K2_SetWorldLocation` (`self.DefaultSceneRoot`) (`self.K2_GetActorLocation` (`self.TargetActor`)) false false)))

(fn `UserConstructionScript`)