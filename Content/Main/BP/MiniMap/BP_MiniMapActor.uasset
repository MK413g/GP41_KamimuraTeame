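; Minimap capture actor that follows player pawn 0 from a fixed height above, using a SceneCaptureComponent2D.
; A Start event fills the capture's show-only list with every actor tagged "MiniMap", and Tick moves the actor each frame.
; SetHidden and SetUnHidden remove or add individual actors in that list at runtime.
; Disconnected leftovers hold an older HiddenActors-based approach.
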(event `Start`
  (bind _outactors (`GameplayStatics.GetAllActorsWithTag` "MiniMap"))
  (set `SceneCaptureComponent.ShowOnlyActors` _outactors (`self.SceneCaptureComponent2D1`)))

(event `self.ReceiveBeginPlay`)

(event `self.ReceiveTick`
  (params (DeltaSeconds :type "Float (single-precision)"))
  (`self.K2_SetActorLocation` (+ (`self.K2_GetActorLocation` (`GameplayStatics.GetPlayerPawn` 0)) (0.0 0.0 1000.0))))

(fn `SetHidden`
  (params (NewItem :type "Actor Object Reference (by ref)"))
  (bind _showonlyactors (`SceneCaptureComponent.ShowOnlyActors` (`self.SceneCaptureComponent2D1`)))
  (if (`KismetArrayLibrary.Array_Contains` _showonlyactors NewItem)
    (`KismetArrayLibrary.Array_RemoveItem` _showonlyactors NewItem)))

(fn `SetUnHidden`
  (params (ItemToFind :type "Actor Object Reference (by ref)"))
  (bind _showonlyactors (`SceneCaptureComponent.ShowOnlyActors` (`self.SceneCaptureComponent2D1`)))
  (if (not (`KismetArrayLibrary.Array_Contains` _showonlyactors ItemToFind))
    (`KismetArrayLibrary.Array_Add` _showonlyactors ItemToFind)))

(fn `UserConstructionScript`)