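; Prologue sequencer that plays the opening cinematic through its camera with background music, then opens the tutorial level.
; Events pause the sequence, create the prologue widget with itself as owner, and change level.
; Skip, gated by a flag, shows a fade, waits, then resets the sequence's frame range to a later section.
; An unconnected chain would set that flag and jump widget narration to its next fixed checkpoint.
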(event `self.ReceiveBeginPlay`
  (`PlayerController.SetViewTargetWithBlend` (`GameplayStatics.GetPlayerController` 0) (`self.Camera`) 0.0 "VTBlend_Linear" 0.0 false)
  (bind (_outactor _returnvalue) (`LevelSequencePlayer.CreateLevelSequencePlayer` "/Game/Main/Sequence/ProlougeSequence/PrologueSequence.PrologueSequence"))
  (bind _output_get (set `self.Sequencer` _returnvalue))
  (`MovieSceneSequencePlayer.Play` _output_get)
  (bind _returnvalue_2 (`GameplayStatics.SpawnSound2D` "/Game/Main/Sound/BGM/Prologue/PrologueBGM_Cue.PrologueBGM_Cue" 1.0 1.0 0.0 null))
  (set `self.soundBGM` _returnvalue_2))

(event `Pause`
  (`MovieSceneSequencePlayer.Pause` (`self.Sequencer`)))

(event `CreateWidget`
  (bind _returnvalue (`|CreateWidget` "/Game/Main/Sequence/ProlougeSequence/PrologueWidget.PrologueWidget_C"))
  (bind _output_get (set `self.widget` _returnvalue))
  (`UserWidget.AddToViewport` _output_get 0)
  (`/Game/Main/Sequence/ProlougeSequence/PrologueWidget.Play` _output_get)
  (`/Game/Main/Sequence/ProlougeSequence/PrologueWidget.SetOwner` _output_get self))

(event `NextLevel`
  (`GameplayStatics.OpenLevelBySoftObjectPtr` "/Game/Main/Level/TutorialLevel.TutorialLevel"))

(event `Key|AnyKey` :consume false
  (params (Key :type "Key Structure")))

(event `Skip`
  ;[1 1 1] アニメーションスキップ処理
  (if (`self.prologueAnimSkip`)
    (bind _returnvalue (`|CreateWidget` "/Game/Main/Sequence/ProlougeSequence/SequencerSkipFade.SequencerSkipFade_C"))
    (`UserWidget.AddToViewport` _returnvalue 0)
    (`/Game/Main/Sequence/ProlougeSequence/SequencerSkipFade.PlayFade` _returnvalue)
    (`KismetSystemLibrary.Delay` 2.5)
    (`MovieSceneSequencePlayer.SetFrameRange` (`self.Sequencer`) 985 1200 0.0)))

(fn `UserConstructionScript`)