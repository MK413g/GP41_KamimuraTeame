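; Epilogue cutscene actor that switches the view to its camera, plays the epilogue Level Sequence and starts the background music.
; Exposed events pause the sequence, play roar and extinction sounds, fade the latter out, and show the epilogue widget.
; Height drives the BPSky sun height, refreshed at construction and through EventSky.
; Once the widget's end flag is set, pressing Jump opens the Title level.
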(event `self.ReceiveBeginPlay`
  (`PlayerController.SetViewTargetWithBlend` (`GameplayStatics.GetPlayerController` 0) (`self.Camera`) 0.0 "VTBlend_Linear" 0.0 false)
  (bind (_outactor _returnvalue) (`LevelSequencePlayer.CreateLevelSequencePlayer` "/Game/Main/Sequence/EpilogueSequence/EpilogueLevelSequence.EpilogueLevelSequence"))
  (bind _output_get (set `self.NewVar_0` _returnvalue))
  (`MovieSceneSequencePlayer.Play` _output_get)
  (bind _returnvalue_2 (`GameplayStatics.SpawnSound2D` "/Game/Main/Sound/BGM/Epilogue/Epilogue_Cue.Epilogue_Cue" 1.0 1.0 0.0 null))
  (set `self.soundBGM` _returnvalue_2))

(event `EventSky`
  (bind _bp_sky (`self.BP_Sky`))
  (set `/Engine/EngineSky/BP_Sky_Sphere.Sun height` (`self.height`) _bp_sky)
  (`/Engine/EngineSky/BP_Sky_Sphere.RefreshMaterial` _bp_sky))

(event `Pause`
  (`MovieSceneSequencePlayer.Pause` (`self.NewVar_0`)))

(event `PlayWidget`
  (bind _returnvalue (`|CreateWidget` "/Game/Main/Sequence/EpilogueSequence/EpilougueWidget.EpilougueWidget_C"))
  (bind _output_get (set `self.Widget` _returnvalue))
  (`UserWidget.AddToViewport` _output_get 0)
  (`/Game/Main/Sequence/EpilogueSequence/EpilougueWidget.PlayEpilogue` _output_get self))

(event `InputAction|Jump`
  (params (Key :type "Key Structure"))
  (bind _widget (`self.Widget`))
  (:`Pressed`
    (`/Engine/EditorBlueprintResources/StandardMacros.IsValid` _widget
      (:`Is Valid`
        (if (`/Game/Main/Sequence/EpilogueSequence/EpilougueWidget.endflg` _widget)
          (`self.NextLevel`))))))

(event `NextLevel`
  (`GameplayStatics.OpenLevelBySoftObjectPtr` "/Game/Main/Level/Title.Title"))

(event `SoundPlayRoar`
  (`SoundManagerBase.PlaySound2D` "/Game/Main/Sound/SE/DragonRoar/DragonRoar_Cur.DragonRoar_Cur" "SE" 1.0 1.0 0.0 null null))

(event `SoundPlayExtinction`
  (bind _returnvalue (`GameplayStatics.SpawnSound2D` "/Game/Main/Sound/SE/EnemyExtinction/EnemyExtinction_Cue.EnemyExtinction_Cue" 1.0 1.0 0.0 null))
  (set `self.soundBus` _returnvalue))

(event `SoundStopExtinction`
  (bind _soundbus (`self.soundBus`))
  (`/Engine/EditorBlueprintResources/StandardMacros.IsValid` _soundbus
    (:`Is Valid`
      (`AudioComponent.FadeOut` _soundbus 2.0 0.0 "Linear"))))

(fn `UserConstructionScript`
  (bind _bp_sky (`self.BP_Sky`))
  (set `/Engine/EngineSky/BP_Sky_Sphere.Sun height` (`self.height`) _bp_sky)
  (`/Engine/EngineSky/BP_Sky_Sphere.RefreshMaterial` _bp_sky))