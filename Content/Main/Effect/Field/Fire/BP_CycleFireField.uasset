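; BP_CycleFireField is a fire field effect that builds a ring of BP_Fire actors one at a time when play begins.
; A custom DelayForLoop macro steps through the indices with a delay between each, and sine and cosine place every spawn evenly around FirePos at FireRadius.
; The loop includes its last index, so the final fire lands on the first one's position.
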(event `self.ReceiveBeginPlay`
  (bind _fire_maxnum (`self.Fire_MaxNum`))
  (bind _fire_radius (`self.Fire_Radius`))
  (bind (_fire_pos_x _fire_pos_y _fire_pos_z) (`KismetMathLibrary.BreakVector` (`self.Fire_Pos`)))
  (bind _index (`self.DelayForLoop` 0 _fire_maxnum (`self.Fire_DelayTime`))
    (:`LoopBody`
      (bind _returnvalue (* _index (/ 360.0 (`KismetMathLibrary.Conv_IntToDouble` _fire_maxnum))))
      (`|SpawnActorFromClass` "/Game/Main/Effect/Field/Fire/BP/BP_Fire.BP_Fire_C" (`KismetMathLibrary.MakeTransform` (`KismetMathLibrary.MakeVector` (+ (* (`KismetMathLibrary.DegCos` _returnvalue) _fire_radius) _fire_pos_x) (+ (* _fire_radius (`KismetMathLibrary.DegSin` _returnvalue)) _fire_pos_y) _fire_pos_z)) "Undefined" "OverrideRootScale" self null))))

(fn `UserConstructionScript`)