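; BP_Laser is a visual laser beam actor that extends along its forward vector and stops at blocking surfaces.
; Each tick, a Visibility line trace sets the Niagara beam's end point and shows the impact effect at the hit location.
; Distance snaps to the hit and grows at BeamSpeed up to MaxDistance, so the beam re-extends gradually once unblocked.
; Both effects take BeamColor on BeginPlay.
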(event `self.ReceiveBeginPlay`
  (`FXSystemComponent.SetColorParameter` (`self.NiagaraLaser`) "Colour" (`self.BeamColor`))
  (`FXSystemComponent.SetColorParameter` (`self.NiagaraLaserImpact`) "Colour" (`self.BeamColor`)))

(event `self.ReceiveTick`
  (params (DeltaSeconds :type "Float (single-precision)"))
  (bind _returnvalue (`self.K2_GetActorLocation`))
  (bind _returnvalue_2 (+ _returnvalue (* (`self.GetActorForwardVector`) (`self.Distance`))))
  (`|ExecutionSequence`
    (:`then_0`
      (set `self.TraceEnd` _returnvalue_2)
      (bind _outhit (`KismetSystemLibrary.LineTraceSingle` _returnvalue _returnvalue_2 "TraceTypeQuery1"))
      (set `self.OnHit` (`GameplayStatics.BreakHitResult` _outhit))
      (set `self.HitLocation` (`.Location` (`GameplayStatics.BreakHitResult` _outhit)))
      (`FXSystemComponent.SetVectorParameter` (`self.NiagaraLaser`) "LaserEnd" (select `bool` (`self.OnHit`) :`false` (`self.TraceEnd`) :`true` (`self.HitLocation`)))
      (`SceneComponent.SetVisibility` (`self.NiagaraLaserImpact`) (`self.OnHit`) false)
      (`SceneComponent.K2_SetWorldLocation` (`self.NiagaraLaserImpact`) (`self.HitLocation`) false false)
      (if (`self.OnHit`)
        (set `self.Distance` (`KismetMathLibrary.VSize` (- (`self.HitLocation`) (`self.K2_GetActorLocation`))))))
    (:`then_1`
      (if (< (`self.Distance`) (`self.MaxDistance`))
        (set `self.Distance` (+ (`self.Distance`) (* DeltaSeconds (`self.BeamSpeed`))))))))

(fn `UserConstructionScript`)