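; BP_Karakasa is the Blueprint for the Karakasa enemy, with placeholder hit-damage handling.
; Each hit on its capsule decrements HP by one.
; It then casts its controller to BP_KarakasaAI and sets the dead flag when HP reaches zero or below.
; It also sets the flinch flag when HP is at or below BeFlinchDamage.
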(event `self.Capsule.OnComponentHit`
  (params (HitComponent :type "PrimitiveComponent Object Reference") (OtherActor :type "Actor Object Reference") (OtherComp :type "PrimitiveComponent Object Reference") (NormalImpulse :type "Vector Structure") (Hit :type "HitResult Structure (by ref)"))
  (bind _asbp_karakasa_ai (cast `/Game/MyFile/ST_EnemyAI/ST_Karakasa/BP_KarakasaAI` (`self.GetController`) :!pure true))
  ;[1 1 1] 被弾(仮)
  (`/Engine/EditorBlueprintResources/StandardMacros.DecrementFloat` (`self.HP`)
    (:`  `
      (`/Game/MyFile/ST_EnemyAI/ST_EnemyAIBase/BP_EnemyBaseAI.SetDeadFlag` _asbp_karakasa_ai (<= (`self.HP`) 0.0))
      (`/Game/MyFile/ST_EnemyAI/ST_EnemyAIBase/BP_EnemyBaseAI.Set Flinch Flag` _asbp_karakasa_ai (<= (`self.HP`) (`self.BeFlinchDamage`))))))

(fn `UserConstructionScript`
  (`parent.UserConstructionScript`))