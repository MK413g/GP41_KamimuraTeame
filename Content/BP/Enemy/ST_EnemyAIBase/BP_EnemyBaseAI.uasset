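; Base enemy AI controller that runs the shared BT_EnemyBaseAI behavior tree when it possesses a pawn.
; Setter functions write flinch, death and player actor blackboard keys, and raising flinch or death calls RunBehaviorTree again on the same tree.
; It stores a per-enemy behavior asset through a getter and setter, but the dynamic subtree injection that would use it is disconnected in this graph.
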(event `self.ReceivePossess`
  (params (PossessedPawn :type "Pawn Object Reference"))
  (`self.RunBehaviorTree` "/Game/MyFile/ST_EnemyAI/ST_EnemyAIBase/BT_EnemyBaseAI.BT_EnemyBaseAI"))

(fn `GetBehavior`
  (returns (NewParam :type "BehaviorTree Object Reference"))
  (return (`self.eachBehavior`)))

(fn `Set Flinch Flag`
  (params (flinch_flag :type Boolean))
  (`BlackboardComponent.SetValueAsBool` (`self.Blackboard`) (`self.Flinch Key Name`) flinch_flag)
  (if flinch_flag
    (`self.RunBehaviorTree` "/Game/MyFile/ST_EnemyAI/ST_EnemyAIBase/BT_EnemyBaseAI.BT_EnemyBaseAI")))

(fn `SetBehavior`
  (params (NewParam :type "BehaviorTree Object Reference"))
  (set `self.eachBehavior` NewParam))

(fn `SetDeadFlag`
  (params (set_flag :type Boolean))
  (`BlackboardComponent.SetValueAsBool` (`self.Blackboard`) (`self.Dead Key Name`) set_flag)
  (if set_flag
    (`self.RunBehaviorTree` "/Game/MyFile/ST_EnemyAI/ST_EnemyAIBase/BT_EnemyBaseAI.BT_EnemyBaseAI")))

(fn `Update PlayerAcyor Key`
  (params (NewParam :type "Actor Object Reference"))
  (`BlackboardComponent.SetValueAsObject` (`self.Blackboard`) (`self.PlayerActor Key Name`) NewParam))

(fn `UserConstructionScript`)